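; Player character with gamepad Enhanced Input for movement and for repositioning an attached ball (Bola) around itself.
; The move input scales walk speed by its dominant axis and moves along actor axes.
; The rotation input computes an unsigned dot-product angle to the stick direction, then Timeline updates rotate the ball's starting offset by that whole angle, without interpolation.
; Unconnected earlier attempts remain: deadzone detection, quadrant-based lerping and physics impulse.
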(event Input|EnhancedActionEvents|EnhancedInputActionIA_myMove
  (params (ActionValue :type Vector%202D%20Structure) (ElapsedSeconds :type Float%20%28double-precision%29) (TriggeredSeconds :type Float%20%28double-precision%29) (InputAction :type Input%20Action%20Object%20Reference :default "/Game/IA_myMove.IA_myMove"))
  (bind _returnvalue (Transformation|GetActorRotation))
  (bind _returnvalue_2 (Transformation|GetActorRotation))
  (bind _charactermovement (Variables|Character|GetCharacterMovement))
  (:Triggered
    (if (> (Math|Float|Absolute(Float) (.x ActionValue)) (Math|Float|Absolute(Float) (.y ActionValue)))
      (Variables|/Script/Engine.CharacterMovementComponent|SetMaxWalkSpeed _charactermovement (Math|Float|Absolute(Float) (* (.x ActionValue) 1.2e+03)))
      (else
        (Variables|/Script/Engine.CharacterMovementComponent|SetMaxWalkSpeed _charactermovement (Math|Float|Absolute(Float) (* (.y ActionValue) 1.2e+03)))))
    (Pawn|Input|AddMovementInput (Math|Vector|GetRightVector (Math|Rotator|MakeRotator (.roll _returnvalue) 0.0 (.yaw _returnvalue))) (.x ActionValue) false)
    (Pawn|Input|AddMovementInput (Math|Vector|GetForwardVector (Math|Rotator|MakeRotator 0.0 (.pitch _returnvalue_2) (.yaw _returnvalue_2))) (.y ActionValue) false)))

(event Input|EnhancedActionEvents|EnhancedInputActionIA_rotacionEsfera
  (params (ActionValue :type Vector%202D%20Structure) (ElapsedSeconds :type Float%20%28double-precision%29) (TriggeredSeconds :type Float%20%28double-precision%29) (InputAction :type Input%20Action%20Object%20Reference :default "/Game/IA_rotacionEsfera.IA_rotacionEsfera"))
  (bind _returnvalue (Math|Vector|Distance2D(Vector) :V1 (Math|Vector2D|MakeVector2D (.x ActionValue) (.y ActionValue))))
  (bind _bola (Variables|Default|Getbola))
  (bind _radio (Variables|Default|Getradio))
  (bind _bola_2 (Variables|Default|Getbola))
  (bind _relativelocation (Variables|/Script/Engine.SceneComponent|GetRelativeLocation _bola_2))
  (bind _relativelocation_2 (Variables|/Script/Engine.SceneComponent|GetRelativeLocation _bola))
  (:Triggered
    (Variables|Default|Setdireccion_x (* (/ (.x ActionValue) _returnvalue) _radio))
    (Variables|Default|Setdireccion_y (* (/ (.y ActionValue) _returnvalue) _radio))
    (Variables|Default|Setdireccion_actual_x (.x _relativelocation_2))
    (Variables|Default|Setdireccion_actual_y (.y _relativelocation_2))
    (Variables|Default|Setangulo%20a%20recoorrer (|(acos((((x1*x2)+(y1*y2))/((sqrt(((square(x1))+(square(y1)))))*(sqrt(((square(x2))+(square(y2))))))))) (.x _relativelocation) (Variables|Default|Getdireccion_x) (.y _relativelocation) (Variables|Default|Getdireccion_y)))
    (Development|PrintString (Utilities|String|ToString(Float) (Variables|Default|Getangulo%20a%20recoorrer)))
    (bind _rotacion (Timeline|Timeline PlayFromStart)
      (:Update
        (Transformation|SetRelativeLocation (Variables|Default|Getbola) (Math|Vector|MakeVector (|((x*(cos(S)))-(y*(sin(S)))) (Variables|Default|Getdireccion_actual_x) (Variables|Default|Getdireccion_actual_y) (|((S*3.141593)/180) (Variables|Default|Getangulo%20a%20recoorrer))) (|((x*(sin(S)))+(y*(cos(S)))) (Variables|Default|Getdireccion_actual_x) (Variables|Default|Getdireccion_actual_y) (|((S*3.141593)/180) (Variables|Default|Getangulo%20a%20recoorrer))) (.z _relativelocation)) false false)))))

(event Collision|EventActorBeginOverlap
  (params (OtherActor :type Actor%20Object%20Reference)))

(event EventTick
  (params (DeltaSeconds :type Float%20%28single-precision%29)))

(event EventBeginPlay
  (bind _asplayer_controller (Utilities|Casting|CastToPlayerController (Pawn|GetController)))
  (Utilities|IsValid (PlayerController|LocalPlayerSubsystems|GetEnhancedInputLocalPlayerSubsystem _asplayer_controller)
    (:Is%20Valid
      (Input|AddMappingContext (PlayerController|LocalPlayerSubsystems|GetEnhancedInputLocalPlayerSubsystem _asplayer_controller) "/Game/controlador_mando.controlador_mando" 0 "(bIgnoreAllPressedKeysUntilRelease=True,bForceImmediately=False)")
      (Development|PrintString (Utilities|String|ToString(Rotator) (Math|Rotator|FindLookatRotation (Math|Vector|MakeVector 1.0 0.0 0.0) (Math|Vector|MakeVector 0.0 1.0 0.0)))))))

(fn ConstructionScript)