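; BP_ProyectileBase is a projectile actor that drains the player's balance (Equilibrio) on hit.
; Its construction script feeds speed, speed limit and gravity variables into ProjectileMovement.
; A Box overlap with a Player-tagged component subtracts balance from BP_Personaje, calling EquilibrioVacio and destroying the projectile only when balance empties.
; With a valid Target, BeginPlay calls Rotate, which just zeroes velocity; the aim-at-target math is unconnected.
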(event OnComponentBeginOverlap(Box)
  (params (OverlappedComponent :type Primitive%20Component%20Object%20Reference) (OtherActor :type Actor%20Object%20Reference) (OtherComp :type Primitive%20Component%20Object%20Reference) (OtherBodyIndex :type Integer) (bFromSweep :type Boolean) (SweepResult :type Hit%20Result%20Structure%20%28by%20ref%29))
  (Development|PrintString "Hello")
  (if (Components|ComponentHasTag OtherComp "Player")
    (bind _asbp_personaje (Utilities|Casting|CastToBP_Personaje OtherActor))
    (bind _output_get (Variables|/Game/Blueprints/BP_Personaje.BP_Personaje_C|SetEquilibrio _asbp_personaje (- (Variables|/Game/Blueprints/BP_Personaje.BP_Personaje_C|GetEquilibrio _asbp_personaje) 1e+02)))
    (if (<= _output_get 0.0)
      (Default|EquilibrioVacio _asbp_personaje)
      (Actor|DestroyActor))))

(event Custom|Rotate
  (Variables|/Script/Engine.MovementComponent|SetVelocity (Variables|Default|GetProjectileMovement) "0, 0, 0"))

(event Collision|EventActorBeginOverlap
  (params (OtherActor :type Actor%20Object%20Reference)))

(event EventTick
  (params (DeltaSeconds :type Float%20%28single-precision%29)))

(event EventBeginPlay
  (Utilities|IsValid (Variables|Default|GetTarget)
    (:Is%20Valid
      (CallFunction|Rotate))))

(fn ConstructionScript
  (bind _projectilemovement (Variables|Default|GetProjectileMovement))
  (Variables|/Script/Engine.ProjectileMovementComponent|SetInitialSpeed _projectilemovement (Variables|ProyectileSettings|GetInitialSpeedP))
  (Variables|/Script/Engine.ProjectileMovementComponent|SetMaxSpeed _projectilemovement (Variables|ProyectileSettings|GetSpeedLimit))
  (Variables|/Script/Engine.ProjectileMovementComponent|SetProjectileGravityScale _projectilemovement (Variables|ProyectileSettings|GetGravedad)))