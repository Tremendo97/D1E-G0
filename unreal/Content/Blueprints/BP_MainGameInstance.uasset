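; Game instance that persists and applies the player's audio and graphics options through a single save slot.
; SaveGame loads or creates a BP_SaveSystem object, writes the volume array and shadow, texture and resolution commands, and runs automatically on shutdown.
; LoadGame reads the slot, then OptionsConfig applies volumes as sound mix overrides for ambient, effects and music classes and runs the stored strings as console commands.
; DeleteSave clears the slot.
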(event Custom|SaveGame
  ;[1 1 1] Guardar
  (Utilities|FlowControl|Sequence
    (:then_0
      (bind _returnvalue (SaveGame|DoesSaveGameExist "SaveSlot1"))
      (if _returnvalue
        (bind _returnvalue_2 (SaveGame|LoadGamefromSlot "SaveSlot1"))
        (bind _asbp_save_system (Utilities|Casting|CastToBP_SaveSystem _returnvalue_2))
        (Variables|Default|SetSaved%20Game%20Ref _asbp_save_system)
        (else
          (bind _returnvalue_3 (SaveGame|CreateSaveGameObject "/Game/Blueprints/BP_SaveSystem.BP_SaveSystem_C"))
          (Variables|Default|SetSaved%20Game%20Ref _returnvalue_3))))
    (:then_1
      (Utilities|IsValid (Variables|Default|GetSaved%20Game%20Ref)
        (:Is%20Valid
          (Variables|/Game/Blueprints/BP_SaveSystem.BP_SaveSystem_C|SetSaveData (Variables|Default|GetSaved%20Game%20Ref) (Utilities|Struct|MakeS_SaveData (Variables|Default|GetVolumeInfo) (Variables|Default|GetCommand%20Shadows) (Variables|Default|GetCommand%20Textures) (Variables|Default|GetCommand%20Resolution)))
          (SaveGame|SaveGametoSlot (Variables|Default|GetSaved%20Game%20Ref) "SaveSlot1"))))))

(event Custom|LoadGame
  ;[1 1 1] Cargar
  (Utilities|FlowControl|Sequence
    (:then_0
      (bind _returnvalue (SaveGame|DoesSaveGameExist "SaveSlot1"))
      (if _returnvalue
        (bind _returnvalue_2 (SaveGame|LoadGamefromSlot "SaveSlot1"))
        (bind _asbp_save_system (Utilities|Casting|CastToBP_SaveSystem _returnvalue_2))
        (Variables|Default|SetSaved%20Game%20Ref _asbp_save_system)))
    (:then_1
      (Utilities|IsValid (Variables|Default|GetSaved%20Game%20Ref)
        (:Is%20Valid
          (CallFunction|OptionsConfig))))))

(event Custom|Options%20config
  (bind _saved_game_ref (Variables|Default|GetSaved%20Game%20Ref))
  (bind _savedata (Variables|/Game/Blueprints/BP_SaveSystem.BP_SaveSystem_C|GetSaveData _saved_game_ref))
  (Utilities|FlowControl|Sequence
    (:then_0
      (Class|GameplayStatics|SetBaseSoundMix "/Game/UI/Sounds/MainSoundMix.MainSoundMix")
      (bind _output_get (Variables|Default|SetVolumeInfo (.volumeinfo _savedata)))
      (for (_array_element _array_index) _output_get
        (switch int _array_index
          (:0
            (Audio|SetSoundMixClassOverride "/Game/UI/Sounds/MainSoundMix.MainSoundMix" "/Game/UI/Sounds/SFX_Ambient.SFX_Ambient" _array_element 1.0 0.0 true))
          (:1
            (Audio|SetSoundMixClassOverride "/Game/UI/Sounds/MainSoundMix.MainSoundMix" "/Game/UI/Sounds/SFX_Effects.SFX_Effects" _array_element 1.0 0.0 true))
          (:2
            (Audio|SetSoundMixClassOverride "/Game/UI/Sounds/MainSoundMix.MainSoundMix" "/Game/UI/Sounds/SFX_Music.SFX_Music" _array_element 1.0 0.0 true)))))
    (:then_1
      (Utilities|FlowControl|Sequence
        (:then_0
          (bind _output_get_2 (Variables|Default|SetCommand%20Shadows (.commandshadows _savedata)))
          (Development|ExecuteConsoleCommand _output_get_2 0))
        (:then_1
          (bind _output_get_3 (Variables|Default|SetCommand%20Textures (.commandtextures _savedata)))
          (Development|ExecuteConsoleCommand _output_get_3 0))
        (:then_2
          (bind _output_get_4 (Variables|Default|SetCommand%20Resolution (.commandresolution _savedata)))
          (Development|ExecuteConsoleCommand _output_get_4 0))))))

(event Custom|DeleteSave
  (bind _returnvalue (SaveGame|DoesSaveGameExist "SaveSlot1"))
  (if _returnvalue
    (SaveGame|DeleteGameinSlot "SaveSlot1")))

(event EventShutdown
  (CallFunction|SaveGame))