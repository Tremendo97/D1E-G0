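; BP_ProyectilMaceta is a flowerpot projectile that homes in on the player.
; It launches forward, then after a second resets velocity, activates particles and homes on its Arrow component, which Tick moves to the player's predicted position using velocity and distance.
; Tick also points the actor at the player.
; On overlap it notifies wheat foliage or dispatches hits by component tag (Player, Escudo, Bola), destroying itself on tagged hits or other untagged components.
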(event OnComponentBeginOverlap(Proyectile)
  (params (OverlappedComponent :type Primitive%20Component%20Object%20Reference) (OtherActor :type Actor%20Object%20Reference) (OtherComp :type Primitive%20Component%20Object%20Reference) (OtherBodyIndex :type Integer) (bFromSweep :type Boolean) (SweepResult :type Hit%20Result%20Structure%20%28by%20ref%29))
  (bind _componenttags (Variables|/Script/Engine.ActorComponent|GetComponentTags OtherComp))
  (if (!= OtherActor (Components|GetOwner))
    (if (Utilities|Array|IsEmpty _componenttags)
      (bind _asinteractive_wheat_foliage (Utilities|Casting|CastToInteractiveWheatFoliage OtherComp)
        (:then
          (Utilities|IsValid _asinteractive_wheat_foliage
            (:Is%20Valid
              (Default|EventHitFoliage _asinteractive_wheat_foliage SweepResult))
            (:Is%20Not%20Valid
              (Actor|DestroyActor :!label _label))))
        (:CastFailed
          (goto _label)))
      (else
        (for _array_element _componenttags
          (switch name _array_element
            (:Player
              (bind _asbp_personaje (Utilities|Casting|CastToBP_Personaje OtherActor))
              (Default|ProjectileHitPersonaje _asbp_personaje)
              (Actor|DestroyActor))
            (:Escudo
              (bind _asbp_escudo_component (Utilities|Casting|CastToBP_Escudo_Component OtherActor))
              (Default|DamageEscudo _asbp_escudo_component)
              (Actor|DestroyActor))
            (:Bola
              (bind _asbp_personaje_2 (Utilities|Casting|CastToBP_Personaje OtherActor))
              (Default|ProjectileHitBola _asbp_personaje_2)
              (Actor|DestroyActor))))))))

(event Custom|Homing
  (bind _projectilemovement (Variables|Default|GetProjectileMovement))
  (Variables|/Script/Engine.ProjectileMovementComponent|SetHomingTargetComponent _projectilemovement (Variables|Default|GetArrow))
  (Variables|/Script/Engine.MovementComponent|SetVelocity _projectilemovement "0, 0, 0")
  (Variables|/Script/Engine.ProjectileMovementComponent|SetbIsHomingProjectile _projectilemovement true)
  (Variables|/Script/Engine.ProjectileMovementComponent|SetHomingAccelerationMagnitude _projectilemovement 3e+03)
  (Components|Activation|Activate (Variables|Default|GetParticleSystem) false))

(event EventTick
  (params (DeltaSeconds :type Float%20%28single-precision%29))
  (bind _returnvalue (Game|GetPlayerCharacter 0))
  (bind _returnvalue_2 (Transformation|GetActorLocation))
  (bind _returnvalue_3 (Game|GetPlayerCharacter 0))
  (bind _arrow (Variables|Default|GetArrow))
  (bind _returnvalue_4 (Transformation|GetActorLocation _returnvalue))
  (bind _returnvalue_5 (Transformation|GetActorLocation _returnvalue_3))
  (bind _returnvalue_6 (Math|Rotator|FindLookatRotation _returnvalue_2 _returnvalue_4))
  (Transformation|SetActorRotation (Math|Rotator|MakeRotator (stale _newtrack_0) (.pitch _returnvalue_6) (.yaw _returnvalue_6)))
  (Utilities|FlowControl|Gate true
    (:Exit
      (Utilities|IsValid _arrow
        (:Is%20Valid
          (Transformation|SetWorldLocation _arrow (+ _returnvalue_5 (* (Pawn|Components|CharacterMovement|GetLastUpdateVelocity (Variables|/Script/Engine.Character|GetCharacterMovement _returnvalue_3)) (/ (Math|Vector|Distance(Vector) (Transformation|GetActorLocation) _returnvalue_5) 2e+03))) false false))))))

(event EventBeginPlay
  (bind _returnvalue (Game|GetPlayerCharacter 0))
  (bind _arrow (Variables|Default|GetArrow))
  (bind _returnvalue_2 (Transformation|GetActorLocation _returnvalue))
  (Game|Components|ProjectileMovement|SetVelocityinLocalSpace (Variables|Default|GetProjectileMovement) "800.000000,0.000000,0.000000")
  (Utilities|FlowControl|Delay 1.0)
  (CallFunction|Homing)
  (Utilities|FlowControl|Gate true) ; enters at Open
)

(fn ConstructionScript
  (bind _projectilemovement (Variables|Default|GetProjectileMovement))
  (Variables|/Script/Engine.ProjectileMovementComponent|SetInitialSpeed _projectilemovement (Variables|ProyectileSettings|GetInitialSpeedP))
  (Variables|/Script/Engine.ProjectileMovementComponent|SetMaxSpeed _projectilemovement (Variables|ProyectileSettings|GetSpeedLimit))
  (Variables|/Script/Engine.ProjectileMovementComponent|SetProjectileGravityScale _projectilemovement (Variables|ProyectileSettings|GetGravedad)))