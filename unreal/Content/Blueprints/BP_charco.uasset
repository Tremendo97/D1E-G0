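; BP_charco is a puddle actor that makes the player slide faster while standing in it.
; Sphere overlap by a "Personaje"-tagged actor raises player 0's BP_Personaje speed and nearly removes ground friction and braking; leaving sets hardcoded normal values.
; The construction script calls crece, whose timeline scales the puddle up from zero, then destroys it after a delay.
; The timeline's Seguir check compares constant vectors, so it never fires.
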(event OnComponentBeginOverlap(Sphere)
  (params (OverlappedComponent :type Primitive%20Component%20Object%20Reference) (OtherActor :type Actor%20Object%20Reference) (OtherComp :type Primitive%20Component%20Object%20Reference) (OtherBodyIndex :type Integer) (bFromSweep :type Boolean) (SweepResult :type Hit%20Result%20Structure%20%28by%20ref%29))
  (Utilities|IsValid OtherActor
    (:Is%20Valid
      (if (Actor|ActorHasTag OtherActor "Personaje")
        (bind _asbp_personaje (Utilities|Casting|CastToBP_Personaje (Game|GetPlayerCharacter 0)))
        (Variables|/Game/Blueprints/BP_Personaje.BP_Personaje_C|SetBase%20Velocity _asbp_personaje 1.2e+03)
        (Variables|/Script/Engine.CharacterMovementComponent|SetGroundFriction (Variables|/Script/Engine.Character|GetCharacterMovement _asbp_personaje) 0.001)
        (Variables|/Script/Engine.CharacterMovementComponent|SetBrakingDecelerationWalking (Variables|/Script/Engine.Character|GetCharacterMovement _asbp_personaje) 0.001)))))

(event OnComponentEndOverlap(Sphere)
  (params (OverlappedComponent :type Primitive%20Component%20Object%20Reference) (OtherActor :type Actor%20Object%20Reference) (OtherComp :type Primitive%20Component%20Object%20Reference) (OtherBodyIndex :type Integer))
  (Utilities|IsValid OtherActor
    (:Is%20Valid
      (if (Actor|ActorHasTag OtherActor "Personaje")
        (bind _asbp_personaje (Utilities|Casting|CastToBP_Personaje (Game|GetPlayerCharacter 0)))
        (Variables|/Game/Blueprints/BP_Personaje.BP_Personaje_C|SetBase%20Velocity _asbp_personaje 8e+02)
        (Variables|/Script/Engine.CharacterMovementComponent|SetGroundFriction (Variables|/Script/Engine.Character|GetCharacterMovement _asbp_personaje) 0.5)
        (Variables|/Script/Engine.CharacterMovementComponent|SetBrakingDecelerationWalking (Variables|/Script/Engine.Character|GetCharacterMovement _asbp_personaje) 2048.0)))))

(event Custom|crece
  (bind (_direction _newtrack_0) (Timeline|Timeline Play)
    (:Update
      (Transformation|SetActorScale3D (Math|Vector|Lerp(Vector) "0, 0, 0" "1.200000,1.200000,1.200000" _newtrack_0))
      (Development|PrintString (Utilities|String|ToString(Vector) "0, 0, 0"))
      (if (Utilities|Operators|EqualEqual :B "1.200000,1.200000,1.200000" :ErrorTolerance 0.1)
        (Variables|Default|Setseguir false)))
    (:Finished
      (switch Utilities|FlowControl|Switch|SwitchonETimelineDirection _direction
        (:Forward
          (Utilities|FlowControl|Delay 7.0)
          (Actor|DestroyActor))))))

(event EventBeginPlay)

(fn ConstructionScript
  (CallFunction|Crece))