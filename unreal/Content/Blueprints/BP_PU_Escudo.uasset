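; BP_PU_Escudo is a shield power-up pickup that gives the player character a shield when touched.
; Its box overlap checks for a Player-tagged component, casts to BP_Personaje, then adds a child actor component of BP_Escudo_Component attached to the character's Bola component before destroying itself.
; The construction script sets the pickup's sphere mesh from its Data asset when valid.
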(event OnComponentBeginOverlap(Box)
  (params (OverlappedComponent :type Primitive%20Component%20Object%20Reference) (OtherActor :type Actor%20Object%20Reference) (OtherComp :type Primitive%20Component%20Object%20Reference) (OtherBodyIndex :type Integer) (bFromSweep :type Boolean) (SweepResult :type Hit%20Result%20Structure%20%28by%20ref%29))
  (if (Components|ComponentHasTag OtherComp "Player")
    (bind _asbp_personaje (Utilities|Casting|CastToBP_Personaje OtherActor))
    (bind _returnvalue (AddComponent|AddChildActorComponent _asbp_personaje true))
    (ChildActorComponent|SetChildActorClass _returnvalue "/Game/Blueprints/BP_Escudo_Component.BP_Escudo_Component_C")
    (Transformation|AttachComponentToComponent _returnvalue (Variables|/Game/Blueprints/BP_Personaje.BP_Personaje_C|Getbola _asbp_personaje) "None" "KeepRelative" "KeepRelative" "KeepRelative" true)
    (Actor|DestroyActor)))

(fn ConstructionScript
  (bind _data (Variables|Default|GetData)
    (:then
      (Components|StaticMesh|SetStaticMesh (Variables|Default|GetSphere) (Variables|/Game/ObjectAndPowerupDataBase/Databases/PDB_Powerups.PDB_Powerups_C|GetMesh _data)))
    (:else)))