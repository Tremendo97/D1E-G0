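; BP_AwaGranja is a hazard volume, apparently farm water by its name, that drains the player's energy while they stay inside its Box.
; Overlap by a component tagged Player opens a Gate and immediately subtracts Energy from BP_MainGameInstance.
; A short Delay feeds back through the Gate to repeat the fixed drain until end overlap closes it.
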(event OnComponentBeginOverlap(Box)
  (params (OverlappedComponent :type Primitive%20Component%20Object%20Reference) (OtherActor :type Actor%20Object%20Reference) (OtherComp :type Primitive%20Component%20Object%20Reference) (OtherBodyIndex :type Integer) (bFromSweep :type Boolean) (SweepResult :type Hit%20Result%20Structure%20%28by%20ref%29))
  (Utilities|IsValid OtherActor
    (:Is%20Valid
      (if (Components|ComponentHasTag OtherComp "Player")
        (Utilities|FlowControl|Sequence
          (:then_0
            (goto _label_2 Open))
          (:then_1
            (bind _asbp_main_game_instance (Utilities|Casting|CastToBP_MainGameInstance (Game|GetGameInstance)))
            (Variables|/Game/Blueprints/BP_MainGameInstance.BP_MainGameInstance_C|SetEnergy _asbp_main_game_instance (- (Variables|/Game/Blueprints/BP_MainGameInstance.BP_MainGameInstance_C|GetEnergy _asbp_main_game_instance) 2.0) :!label _label)
            (Utilities|FlowControl|Delay 0.1)
            (Utilities|FlowControl|Gate false :!label _label_2
              (:Exit
                (goto _label)))))))))

(event OnComponentEndOverlap(Box)
  (params (OverlappedComponent :type Primitive%20Component%20Object%20Reference) (OtherActor :type Actor%20Object%20Reference) (OtherComp :type Primitive%20Component%20Object%20Reference) (OtherBodyIndex :type Integer))
  (Utilities|IsValid OtherActor
    (:Is%20Valid
      (if (Components|ComponentHasTag OtherComp "Player")
        (Utilities|FlowControl|Gate false) ; enters at Close
      ))))

(fn ConstructionScript)