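; BP_salidas is a level exit that triggers once when the player overlaps its box with at least two Dominados.
; It stuns all, stops damage and music, fires four Niagara effects and spins the column via a timeline, then after a delay loads the next level by current level name (City to Granja to Astillero).
; In Lvl_AstilleroPrueba it instead shows the win widget and pauses the game.
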(event OnComponentBeginOverlap(Box)
  (params (OverlappedComponent :type Primitive%20Component%20Object%20Reference) (OtherActor :type Actor%20Object%20Reference) (OtherComp :type Primitive%20Component%20Object%20Reference) (OtherBodyIndex :type Integer) (bFromSweep :type Boolean) (SweepResult :type Hit%20Result%20Structure%20%28by%20ref%29))
  (Utilities|IsValid OtherActor
    (:Is%20Valid
      (if (Components|ComponentHasTag OtherComp "Player")
        (bind _asbp_personaje (Utilities|Casting|CastToBP_Personaje (Game|GetPlayerCharacter 0)))
        (if (>= (Variables|/Game/Blueprints/BP_Personaje.BP_Personaje_C|Getdominados _asbp_personaje) 2)
          (Utilities|FlowControl|DoOnce false
            (:Completed
              (bind _asbp_main_game_instance (Utilities|Casting|CastToBP_MainGameInstance (Game|GetGameInstance)))
              (if (Utilities|Enum|Equal(Enum) (Utilities|String|ToString(Name) (Variables|/Game/Blueprints/BP_MainGameInstance.BP_MainGameInstance_C|GetCurrentLevel _asbp_main_game_instance)) "Lvl_AstilleroPrueba")
                (bind _returnvalue (UserInterface|CreateWidget "/Game/UI/W_win.W_win_C"))
                (bind _output_get (Variables|Default|Setwin _returnvalue))
                (UserInterface|Viewport|AddtoViewport _output_get 0)
                (Game|SetGamePaused true)
                (else
                  (Default|StunAll _asbp_personaje)
                  (Default|StopDamage _asbp_personaje)
                  (Default|StopMusic (Variables|/Game/Blueprints/BP_Personaje.BP_Personaje_C|GetHUD _asbp_personaje))
                  (Variables|/Game/Blueprints/BP_Personaje.BP_Personaje_C|SetStunned _asbp_personaje true)
                  (Components|Activation|Activate (Variables|Default|GetNS_Salida1) true)
                  (CallFunction|GirarColumnas)
                  (Utilities|FlowControl|Delay 4.0)
                  (bind _asbp_main_game_instance_2 (Utilities|Casting|CastToBP_MainGameInstance (Game|GetGameInstance)))
                  (switch string (Utilities|String|ToString(Name) (Variables|/Game/Blueprints/BP_MainGameInstance.BP_MainGameInstance_C|GetCurrentLevel _asbp_main_game_instance_2))
                    (:Lvl_CityMitadTam
                      (Default|EventLoadLevel _asbp_main_game_instance_2 "Lvl_Granja"))
                    (:Lvl_Granja
                      (Default|EventLoadLevel _asbp_main_game_instance_2 "Lvl_AstilleroPrueba"))))))))))))

(event Custom|GirarColumnas
  (Rendering|Material|SetMaterial (Variables|Default|GetBase) 1 "/Game/Materials/M_CargaRadial.M_CargaRadial")
  (bind _1 (Timeline|Rotator Play)
    (:Update
      (Transformation|SetRelativeRotation (Variables|Default|GetColumna) (Math|Rotator|Lerp(Rotator) "0, 0, 0" "0.000000,720.000000,0.000000" _1) false false))))

(event EventBeginPlay
  (Components|Activation|Deactivate (Variables|Default|GetNS_Salida1))
  (Components|Activation|Deactivate (Variables|Default|GetNS_Salida2))
  (Components|Activation|Deactivate (Variables|Default|GetNS_Salida3))
  (Components|Activation|Deactivate (Variables|Default|GetNS_Salida4)))

(fn ConstructionScript)