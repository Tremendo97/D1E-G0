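; Spinning pickup that grants the player a random power-up: an ability, a shield, or a movement or rotation speed boost.
; On the first overlap by a Player-tagged component, it shuffles the GameInstance's PowerUps pool and applies the first entry.
; It shows a WBP_PowerUp message, stores the upgrade in the GameInstance and updates BP_Personaje where needed.
; It then removes that entry, except rotating shields while their count stays below three, and destroys itself.
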(event OnComponentBeginOverlap(Box)
  (params (OverlappedComponent :type Primitive%20Component%20Object%20Reference) (OtherActor :type Actor%20Object%20Reference) (OtherComp :type Primitive%20Component%20Object%20Reference) (OtherBodyIndex :type Integer) (bFromSweep :type Boolean) (SweepResult :type Hit%20Result%20Structure%20%28by%20ref%29))
  (Utilities|IsValid OtherActor
    (:Is%20Valid
      (if (Components|ComponentHasTag OtherComp "Player")
        (Utilities|FlowControl|DoOnce false
          (:Completed
            (bind _returnvalue (UserInterface|CreateWidget "/Game/UI/WBP_PowerUp.WBP_PowerUp_C"))
            (bind _output_get (Variables|Default|SetUI _returnvalue))
            (UserInterface|Viewport|AddtoViewport _output_get 0)
            (bind _asbp_main_game_instance (Utilities|Casting|CastToBP_MainGameInstance (Game|GetGameInstance)))
            (bind _output_get_2 (Variables|Default|SetGame%20Instance%20Ref _asbp_main_game_instance))
            (Utilities|Array|Shuffle (Variables|/Game/Blueprints/BP_MainGameInstance.BP_MainGameInstance_C|GetPowerUps _output_get_2))
            (Utilities|FlowControl|Sequence
              (:then_0
                (switch Utilities|FlowControl|Switch|SwitchonE_PowerUps (Utilities|Array|Get(acopy) (Variables|/Game/Blueprints/BP_MainGameInstance.BP_MainGameInstance_C|GetPowerUps _output_get_2))
                  (:NewEnumerator0
                    (Default|ShowMessage (Variables|Default|GetUI) "DECOY" "Pulsa F (X en mando) para distraer a los enemigos")
                    (Variables|/Game/Blueprints/BP_MainGameInstance.BP_MainGameInstance_C|SetHas_PU_Ardilla (Variables|Default|GetGame%20Instance%20Ref) true))
                  (:NewEnumerator1
                    (Default|ShowMessage (Variables|Default|GetUI) "ESCUDO" "Efecto pasivo 
Previene de un golpe 
Se regenera con el tiempo")
                    (Variables|/Game/Blueprints/BP_MainGameInstance.BP_MainGameInstance_C|SetHas_PU_Escudo (Variables|Default|GetGame%20Instance%20Ref) true)
                    (bind _asbp_personaje (Utilities|Casting|CastToBP_Personaje (Game|GetPlayerCharacter 0)))
                    (Default|SetEscudo _asbp_personaje))
                  (:NewEnumerator2
                    (Default|ShowMessage (Variables|Default|GetUI) "RANGO" "Mantén RMB (RT en mando) para aumentar el radio de giro")
                    (Variables|/Game/Blueprints/BP_MainGameInstance.BP_MainGameInstance_C|SetHas_PU_Rango (Variables|Default|GetGame%20Instance%20Ref) true))
                  (:NewEnumerator3
                    (Default|ShowMessage (Variables|Default|GetUI) "TASER" "Pulsa R (Circulo en mando) para stunear a los enemigos cercanos")
                    (Variables|/Game/Blueprints/BP_MainGameInstance.BP_MainGameInstance_C|SetHas_PU_Stunner (Variables|Default|GetGame%20Instance%20Ref) true))
                  (:NewEnumerator4
                    (Default|ShowMessage (Variables|Default|GetUI) "ZAPATILLAS" "Aumenta ligeramente la velocidad de movimiento")
                    (bind _output_get_3 (Variables|/Game/Blueprints/BP_MainGameInstance.BP_MainGameInstance_C|SetMax%20Walk%20Speed (Variables|Default|GetGame%20Instance%20Ref) (+ (Variables|/Game/Blueprints/BP_MainGameInstance.BP_MainGameInstance_C|GetMax%20Walk%20Speed (Variables|Default|GetGame%20Instance%20Ref)) 1e+02)))
                    (bind _asbp_personaje_2 (Utilities|Casting|CastToBP_Personaje (Game|GetPlayerCharacter 0)))
                    (Variables|/Game/Blueprints/BP_Personaje.BP_Personaje_C|SetBase%20Velocity _asbp_personaje_2 _output_get_3))
                  (:NewEnumerator5
                    (Default|ShowMessage (Variables|Default|GetUI) "PROPULSORES" "Aumenta significativamente la velocidad de movimiento")
                    (bind _output_get_4 (Variables|/Game/Blueprints/BP_MainGameInstance.BP_MainGameInstance_C|SetMax%20Walk%20Speed (Variables|Default|GetGame%20Instance%20Ref) (+ (Variables|/Game/Blueprints/BP_MainGameInstance.BP_MainGameInstance_C|GetMax%20Walk%20Speed (Variables|Default|GetGame%20Instance%20Ref)) 3e+02)))
                    (bind _asbp_personaje_3 (Utilities|Casting|CastToBP_Personaje (Game|GetPlayerCharacter 0)))
                    (Variables|/Game/Blueprints/BP_Personaje.BP_Personaje_C|SetBase%20Velocity _asbp_personaje_3 _output_get_4))
                  (:NewEnumerator6
                    (Default|ShowMessage (Variables|Default|GetUI) "GIROSCOPIO" "Aumenta ligeramente la velocidad de rotación de la célula de energía")
                    (bind _output_get_5 (Variables|/Game/Blueprints/BP_MainGameInstance.BP_MainGameInstance_C|SetRotation%20Speed (Variables|Default|GetGame%20Instance%20Ref) (+ (Variables|/Game/Blueprints/BP_MainGameInstance.BP_MainGameInstance_C|GetRotation%20Speed (Variables|Default|GetGame%20Instance%20Ref)) 1e+04)))
                    (bind _asbp_personaje_4 (Utilities|Casting|CastToBP_Personaje (Game|GetPlayerCharacter 0)))
                    (Variables|/Game/Blueprints/BP_Personaje.BP_Personaje_C|Setvelocidad%20tangencial _asbp_personaje_4 _output_get_5))
                  (:NewEnumerator7
                    (Default|ShowMessage (Variables|Default|GetUI) "MÓDULO GRAVITACIONAL" "Aumenta significativamente la velocidad de rotación de la célula de energía")
                    (bind _output_get_6 (Variables|/Game/Blueprints/BP_MainGameInstance.BP_MainGameInstance_C|SetRotation%20Speed (Variables|Default|GetGame%20Instance%20Ref) (+ (Variables|/Game/Blueprints/BP_MainGameInstance.BP_MainGameInstance_C|GetRotation%20Speed (Variables|Default|GetGame%20Instance%20Ref)) 2e+04)))
                    (bind _asbp_personaje_5 (Utilities|Casting|CastToBP_Personaje (Game|GetPlayerCharacter 0)))
                    (Variables|/Game/Blueprints/BP_Personaje.BP_Personaje_C|Setvelocidad%20tangencial _asbp_personaje_5 _output_get_6))
                  (:NewEnumerator8
                    (Default|ShowMessage (Variables|Default|GetUI) "ESCUDO ROTATORIO" "Usa Los escudos para protegerte de algunos golpes. puedes llegar a tener 3 que giren junto a la bola.")
                    (bind _asbp_personaje_6 (Utilities|Casting|CastToBP_Personaje (Game|GetPlayerCharacter 0)))
                    (Default|ActivateEscudosRotatorios _asbp_personaje_6)
                    (bind _output_get_7 (Variables|/Game/Blueprints/BP_MainGameInstance.BP_MainGameInstance_C|SetnumEscudosRota _asbp_main_game_instance (+ (Variables|/Game/Blueprints/BP_MainGameInstance.BP_MainGameInstance_C|GetnumEscudosRota _asbp_main_game_instance) 1)))
                    (if (< _output_get_7 3)
                      (Variables|Default|Setrotatorios true)))))
              (:then_1
                (if (Variables|Default|Getrotatorios)
                  (Variables|Default|Setrotatorios false)
                  (else
                    (Utilities|Array|RemoveIndex (Variables|/Game/Blueprints/BP_MainGameInstance.BP_MainGameInstance_C|GetPowerUps _output_get_2))))
                (Actor|DestroyActor)))))))))

(event EventTick
  (params (DeltaSeconds :type Float%20%28single-precision%29))
  (Transformation|AddLocalRotation (Variables|Default|GetStaticMesh) "0.400000,0.600000,0.500000" false false)
  (Transformation|AddLocalRotation (Variables|Default|GetStaticMesh1) "0.000000,0.500000,0.000000" false false))

(fn ConstructionScript)