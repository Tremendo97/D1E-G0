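; Enemy Blueprint with an attack that fires BP_ProyectileBase from its location along the Scene component's rotation.
; Attack calls SetAim5º, waits briefly, then spawns; a Spawn Proyectile function variant adds a yaw offset.
; Aim events write a look-at direction vector into Weapon's world location, not rotation, and SetAim5º adds 90° yaw despite its name.
; BeginPlay calls an empty ChasePlayer, as its AIMoveTo loop is disconnected.
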(event Custom|ChasePlayer)

(event Custom|Attack
  (CallFunction|SetAim5º)
  (Utilities|FlowControl|Delay 0.2)
  (CallFunction|SpawnProyectile))

(event Custom|SpawnProyectile
  (bind _scene (Variables|Default|GetScene))
  (bind _returnvalue (Transformation|GetWorldRotation _scene))
  (Game|SpawnActorfromClass "/Game/Blueprints/BP_ProyectileBase.BP_ProyectileBase_C" (Math|Transform|MakeTransform (Transformation|GetActorLocation) (Math|Rotator|MakeRotator (.roll _returnvalue) (.pitch _returnvalue) (.yaw _returnvalue))) "AlwaysSpawn" "MultiplyWithRoot" 0 0))

(event Custom|SetAim5º
  (bind _returnvalue (Game|Player|GetPlayerPawn 0))
  (bind _weapon (Variables|Default|GetWeapon))
  (bind _returnvalue_2 (Transformation|GetWorldLocation _weapon))
  (bind _returnvalue_3 (Transformation|GetActorLocation _returnvalue))
  (bind _returnvalue_4 (Math|Rotator|FindLookatRotation _returnvalue_2 _returnvalue_3))
  (bind (_roll _pitch _yaw) (Math|Rotator|BreakRotator _returnvalue_4))
  ;[1 1 1] Look5º
  (Transformation|SetWorldLocation (Variables|Default|GetWeapon) (Math|Rotator|GetRotationXVector (Math|Rotator|MakeRotator 0.0 _pitch (+ _yaw 9e+01))) false false))

(event Custom|SetAim
  (bind _returnvalue (Game|Player|GetPlayerPawn 0))
  (bind _weapon (Variables|Default|GetWeapon))
  (bind _returnvalue_2 (Transformation|GetWorldLocation _weapon))
  (bind _returnvalue_3 (Transformation|GetActorLocation _returnvalue))
  (bind _returnvalue_4 (Math|Rotator|FindLookatRotation _returnvalue_2 _returnvalue_3))
  (bind (_roll _pitch _yaw) (Math|Rotator|BreakRotator _returnvalue_4))
  ;[1 1 1] Look
  (Transformation|SetWorldLocation (Variables|Default|GetWeapon) (Math|Rotator|GetRotationXVector (Math|Rotator|MakeRotator 0.0 _pitch _yaw)) false false))

(event EventBeginPlay
  (CallFunction|ChasePlayer))

(event Collision|EventActorBeginOverlap
  (params (OtherActor :type Actor%20Object%20Reference)))

(event EventTick
  (params (DeltaSeconds :type Float%20%28single-precision%29)))

(fn ConstructionScript)

(fn SpawnProyectile
  (params (DiferenciaAnguloSpawn :type Float%20%28double-precision%29))
  (bind _scene (Variables|Default|GetScene))
  (bind _returnvalue (Transformation|GetWorldRotation _scene))
  (Game|SpawnActorfromClass "/Game/Blueprints/BP_ProyectileBase.BP_ProyectileBase_C" (Math|Transform|MakeTransform (Transformation|GetActorLocation) (Math|Rotator|MakeRotator (.roll _returnvalue) (.pitch _returnvalue) (+ (.yaw _returnvalue) DiferenciaAnguloSpawn))) "AlwaysSpawn" "MultiplyWithRoot" 0 0))