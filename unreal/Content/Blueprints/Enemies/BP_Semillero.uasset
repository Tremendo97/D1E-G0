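; BP_Semillero is an enemy Blueprint that steers its AI target through the "Attack" Blackboard key and disturbs wheat foliage it touches.
; When a squirrel (Ardilla) creation event fires, that squirrel becomes the Attack target, and its EndPlay switches the key to the player character.
; Overlaps on SemilleroBase forward the sweep result to interactive wheat foliage components through their hit event.
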(event OnComponentBeginOverlap(SemilleroBase)
  (params (OverlappedComponent :type Primitive%20Component%20Object%20Reference) (OtherActor :type Actor%20Object%20Reference) (OtherComp :type Primitive%20Component%20Object%20Reference) (OtherBodyIndex :type Integer) (bFromSweep :type Boolean) (SweepResult :type Hit%20Result%20Structure%20%28by%20ref%29))
  (bind _asinteractive_wheat_foliage (Utilities|Casting|CastToInteractiveWheatFoliage OtherComp))
  (Utilities|IsValid _asinteractive_wheat_foliage
    (:Is%20Valid
      (Default|EventHitFoliage _asinteractive_wheat_foliage SweepResult))))

(event Custom|On%20Crear%20Ardilla
  (params (Ardilla%20Reference :type BP%20Ardilla%20Object%20Reference))
  (Game|BindEventtoOnEndPlay Ardilla%20Reference (delegate Custom|CustomEvent))
  (AI|Components|Blackboard|SetValueasObject (AI|GetBlackboard 0) (Utilities|Name|MakeLiteralName "Attack") Ardilla%20Reference))

(event Custom|CustomEvent
  (params (Actor :type Actor%20Object%20Reference) (EndPlayReason :type EEndPlayReason%20Enum :default "Destroyed"))
  (AI|Components|Blackboard|SetValueasObject (AI|GetBlackboard 0) (Utilities|Name|MakeLiteralName "Attack") (Game|GetPlayerCharacter 0)))

(fn ConstructionScript)