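; Enemy wheel character that patrols random navigable points around itself and charges at the player on sight.
; PawnSensing triggers a DoOnce sequence that stops movement, turns to face the player for a short wind-up, then rushes slightly past the player's recorded position.
; After the charge it resets detection, slows down, pauses and resumes patrolling.
; Hitting an actor tagged Personaje launches the player forward and upward.
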(event OnSeePawn(PawnSensing)
  (params (Pawn :type Pawn%20Object%20Reference))
  (bind _charactermovement (Variables|Character|GetCharacterMovement))
  ;[1 1 1] Secuencia de comportamiento
  (Utilities|FlowControl|DoOnce false
    (:Completed
      (Variables|Default|SetMoveRandom false)
      (Utilities|FlowControl|Sequence
        (:then_0
          (Pawn|Components|CharacterMovement|DisableMovement _charactermovement))
        (:then_1
          (Variables|/Script/Engine.CharacterMovementComponent|SetMaxWalkSpeed _charactermovement 1e+03))
        (:then_2
          (CallFunction|Charge))))))

(event Custom|ResetDoOnce
  (bind _charactermovement (Variables|Character|GetCharacterMovement))
  ;[1 1 1] Secuencia de comportamiento
  (Utilities|FlowControl|DoOnce false) ; enters at Reset
)

(event Custom|MoveToRandomLocation
  ;[1 1 1] Rueda patrulla (movimiento aleatorio en un radio)
  (if (Variables|Default|GetMoveRandom)
    (bind _randomlocation (Class|NavigationSystemV1|GetRandomLocationinNavigableRadius (Transformation|GetActorLocation) 1e+03 0 0))
    (AI|AIMoveTo self _randomlocation 0 5.0 false
      (:then
        (Utilities|FlowControl|Delay 2.0)
        (CallFunction|MovetoRandomLocation)))))

(event Custom|Charge
  (bind _self self)
  (bind _returnvalue (Transformation|GetActorLocation _self))
  ;[1 1 1] Charge/Placaje
  (Variables|Default|SetSetAim true)
  (Utilities|FlowControl|Delay 2.0)
  (Pawn|Components|CharacterMovement|SetMovementMode (Variables|Character|GetCharacterMovement) "MOVE_Walking" 0)
  (Variables|Default|SetPlayerPosition (Transformation|GetActorLocation (Game|GetPlayerCharacter 0)))
  (Variables|Default|SetSetAim false)
  (AI|AIMoveTo self (+ (* (Math|Vector|Normalize (- (Variables|Default|GetPlayerPosition) _returnvalue)) (+ (Math|Vector|Distance(Vector) _returnvalue (Variables|Default|GetPlayerPosition)) 2e+02)) (Transformation|GetActorLocation self)) 0 5.0 false
    (:OnSuccess
      _)
    (:OnFail
      (Utilities|FlowControl|Delay 0.2)))
  (CallFunction|ResetDoOnce)
  (Variables|/Script/Engine.CharacterMovementComponent|SetMaxWalkSpeed (Variables|Character|GetCharacterMovement) 4e+02)
  (Utilities|FlowControl|RetriggerableDelay 3.0)
  (Variables|Default|SetMoveRandom true)
  (CallFunction|MovetoRandomLocation))

(event EventBeginPlay
  ;[1 1 1] Rueda patrulla (movimiento aleatorio en un radio)
  (CallFunction|MovetoRandomLocation))

(event EventTick
  (params (DeltaSeconds :type Float%20%28single-precision%29))
  ;[1 1 1] Face Player (SetAim)
  (if (Variables|Default|GetSetAim)
    (Transformation|SetActorRotation (Math|Rotator|MakeRotator 0.0 0.0 (.yaw (Math|Rotator|FindLookatRotation (Transformation|GetActorLocation) (Transformation|GetActorLocation (Game|Player|GetPlayerPawn 0))))))))

(event Collision|EventHit
  (params (MyComp :type Primitive%20Component%20Object%20Reference) (Other :type Actor%20Object%20Reference) (OtherComp :type Primitive%20Component%20Object%20Reference) (bSelfMoved :type Boolean) (HitLocation :type Vector :default "0, 0, 0") (HitNormal :type Vector :default "0, 0, 0") (NormalImpulse :type Vector :default "0, 0, 0") (Hit :type Hit%20Result%20Structure%20%28by%20ref%29))
  (bind _returnvalue (Transformation|GetActorForwardVector))
  ;[1 1 1] Empujar al jugador
  (if (Actor|ActorHasTag (.HitActor (Collision|BreakHitResult Hit)) "Personaje")
    (Character|LaunchCharacter (Game|GetPlayerCharacter 0) (Math|Vector|MakeVector (* (.x _returnvalue) 8e+02) (* (.y _returnvalue) 8e+02) 5e+02) true true)))

(fn ConstructionScript)