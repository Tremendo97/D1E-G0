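; Semillero enemy Blueprint with a tracks material and a function that fires projectiles from its spawn arrow, driven by AI blackboard keys.
; It binds to player events: a spawned squirrel (Ardilla) becomes the Attack target until its end play, and a pulse within range sets stunned for a retriggerable duration.
; Its capsule triggers hit reactions on interactive wheat foliage.
; SpawnProyectile ignores its angle inputs and still prints a debug string.
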(event OnComponentBeginOverlap(CapsuleComponent)
  (params (OverlappedComponent :type Primitive%20Component%20Object%20Reference) (OtherActor :type Actor%20Object%20Reference) (OtherComp :type Primitive%20Component%20Object%20Reference) (OtherBodyIndex :type Integer) (bFromSweep :type Boolean) (SweepResult :type Hit%20Result%20Structure%20%28by%20ref%29))
  ;[1 0.9398 0.3352] Pisar Trigo
  (bind _asinteractive_wheat_foliage (Utilities|Casting|CastToInteractiveWheatFoliage OtherComp))
  (Utilities|IsValid _asinteractive_wheat_foliage
    (:Is%20Valid
      (Default|EventHitFoliage _asinteractive_wheat_foliage SweepResult))))

(event Custom|pulso
  (params (Tiempo :type Float%20%28double-precision%29) (Distancia :type Float%20%28double-precision%29))
  (if (<= (Math|Vector|Distance(Vector) (Transformation|GetActorLocation (Game|GetPlayerCharacter 0)) (Transformation|GetActorLocation)) Distancia)
    (AI|Components|Blackboard|SetValueasBool (AI|GetBlackboard 0) (Utilities|Name|MakeLiteralName "stunned") true)
    (Utilities|FlowControl|RetriggerableDelay Tiempo)
    (AI|Components|Blackboard|SetValueasBool (AI|GetBlackboard 0) (Utilities|Name|MakeLiteralName "stunned") false)))

(event Custom|On%20Crear%20Ardilla
  (params (Arilla%20Reference :type BP%20Ardilla%20Object%20Reference))
  ;[1 0.5616 0.3172] Ardilla
  (Game|BindEventtoOnEndPlay Arilla%20Reference (delegate Custom|CustomEvent))
  (AI|Components|Blackboard|SetValueasObject (AI|GetBlackboard 0) (Utilities|Name|MakeLiteralName "Attack") Arilla%20Reference))

(event Custom|CustomEvent
  (params (Actor :type Actor%20Object%20Reference) (EndPlayReason :type EEndPlayReason%20Enum :default "Destroyed"))
  (bind _returnvalue (AI|GetBlackboard 0))
  ;[1 0.5616 0.3172] Ardilla
  (Game|UnbindEventfromOnEndPlay Actor (delegate Custom|CustomEvent))
  (Utilities|IsValid _returnvalue
    (:Is%20Valid
      (AI|Components|Blackboard|SetValueasObject _returnvalue (Utilities|Name|MakeLiteralName "Attack") (Game|GetPlayerCharacter 0)))))

(event EventBeginPlay
  (bind _asbp_personaje (Utilities|Casting|CastToBP_Personaje (Game|GetPlayerCharacter 0)))
  (EventDispatchers|BindEventtoCrearArdilla _asbp_personaje (delegate Custom|On%20Crear%20Ardilla))
  (EventDispatchers|BindEventtoPulso _asbp_personaje (delegate Custom|pulso)))

(fn ConstructionScript
  (bind _returnvalue (Rendering|Material|CreateDynamicMaterialInstance (Variables|Default|GetSemillero_Tracks) 0 "/Game/Materials/M_Enemigos/MI_Tracks_Semillero.MI_Tracks_Semillero" "None" :!class /Script/Engine.PrimitiveComponent))
  (Variables|Default|SetTracks _returnvalue))

(fn SpawnProyectile
  (params (DiferenciaAnguloSpawn :type Float%20%28double-precision%29) (Subida%20angulo :type Float%20%28double-precision%29))
  (bind _spawnarrow (Variables|Default|GetSpawnArrow))
  (bind _returnvalue (Transformation|GetWorldLocation _spawnarrow))
  (bind _returnvalue_2 (Transformation|GetWorldRotation _spawnarrow))
  (bind _returnvalue_3 (Math|Transform|MakeTransform _returnvalue _returnvalue_2))
  (Development|PrintString "Hello")
  (Game|SpawnActorfromClass "/Game/Blueprints/BP_ProyectileBase.BP_ProyectileBase_C" (Math|Transform|MakeTransform (.location _returnvalue_3) (.rotation _returnvalue_3) (.scale _returnvalue_3)) "AlwaysSpawn" "MultiplyWithRoot" 0 0))