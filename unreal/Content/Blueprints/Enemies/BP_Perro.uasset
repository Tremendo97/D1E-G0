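; BP_Perro is a wheeled dog character in the Enemies folder that targets and collects energy objects the player creates.
; Player energy-creation and death events maintain a queue, feeding its first entry to the Blackboard "Target" key.
; Collecting opens the jaw via timeline and raises an energy bar drawn through a dynamic material.
; It also offers a timed Blackboard stun and angle-offset projectile spawning, while sight handling is an empty stub.
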(event Custom|On%20Energy%20Created
  (params (Energy%20Reference :type BP%20Energia%20Object%20Reference))
  (bind _energyarray (Variables|Default|GetEnergyArray))
  ;[0 252 5000] Energy
  (Utilities|Array|Add _energyarray Energy%20Reference)
  (EventDispatchers|BindEventtoMuerteEnegia Energy%20Reference (delegate Custom|On%20Energy%20Destroyed))
  (if (== (Utilities|Array|Length _energyarray) 1)
    (AI|Components|Blackboard|SetValueasObject (AI|GetBlackboard 0) (Utilities|Name|MakeLiteralName "Target") Energy%20Reference)))

(event Custom|On%20Energy%20Destroyed
  (params (Energy%20Reference :type BP%20Energia%20Object%20Reference))
  (bind _energyarray (Variables|Default|GetEnergyArray))
  ;[0 252 5000] Energy
  (EventDispatchers|UnbindEventfromMuerteEnegia Energy%20Reference (delegate Custom|On%20Energy%20Destroyed))
  (Utilities|Array|RemoveItem _energyarray Energy%20Reference)
  (if (Utilities|Array|IsEmpty _energyarray)
    (AI|Components|Blackboard|ClearValue (AI|GetBlackboard 0) (Utilities|Name|MakeLiteralName "Target"))
    (else
      (AI|Components|Blackboard|SetValueasObject (AI|GetBlackboard 0) (Utilities|Name|MakeLiteralName "Target") (Utilities|Array|Get(acopy) _energyarray)))))

(event Custom|RecogerEnergia
  ;[1 0.7084 0] Open mouth y Progress Bar Energía
  (Utilities|FlowControl|Sequence
    (:then_0
      (bind _rotation (Timeline|OpenMouth Play)
        (:Update
          (Transformation|SetRelativeRotation (Variables|Default|GetPerro_Cabeza) (Math|Rotator|MakeRotator (Math|Float|Lerp 0.0 -6e+01 _rotation) 0.0 -9e+01) false false))))
    (:then_1
      (Utilities|FlowControl|Delay 0.8)
      (Timeline|OpenMouth Reverse))
    (:then_2
      (bind _output_get (Variables|Default|SetProgressBarEnergia (+ (Variables|Default|GetProgressBarEnergia) 0.05)))
      (Rendering|Material|SetScalarParameterValue (Variables|Default|GetProgressBarMaterialInstance) "ProgressBarEnergia" _output_get :!class /Script/Engine.MaterialInstanceDynamic))))

(event EventStunn
  (params (tiempo :type Float%20%28double-precision%29))
  (AI|Components|Blackboard|SetValueasBool (AI|GetBlackboard (AI|GetAIController self)) (Utilities|Name|MakeLiteralName "stunned") true)
  (Utilities|FlowControl|RetriggerableDelay tiempo)
  (AI|Components|Blackboard|SetValueasBool (AI|GetBlackboard (AI|GetAIController self)) (Utilities|Name|MakeLiteralName "stunned") false))

(event EventBeginPlay
  (bind _asbp_personaje (Utilities|Casting|CastToBP_Personaje (Game|GetPlayerCharacter 0)))
  (EventDispatchers|BindEventtoCrearEnergia _asbp_personaje (delegate Custom|On%20Energy%20Created)))

(fn ConstructionScript
  (bind _returnvalue (Rendering|Material|CreateDynamicMaterialInstance (Variables|Default|GetPerro_Cuerpo) 1 "/Game/Materials/Enemigos/M_ProgressBarEnergia_Perro.M_ProgressBarEnergia_Perro" "None" :!class /Script/Engine.PrimitiveComponent))
  (Variables|Default|SetProgressBarMaterialInstance _returnvalue)
  (bind _returnvalue_2 (Rendering|Material|CreateDynamicMaterialInstance (Variables|Default|GetPerro_Rueda) 0 "/Game/Materials/Enemigos/MI_Tracks_Perrro.MI_Tracks_Perrro" "None" :!class /Script/Engine.PrimitiveComponent))
  (bind _output_get (Variables|Default|SetTracks _returnvalue_2))
  (Rendering|Material|SetScalarParameterValue _output_get "XSpeed" 0.0 :!class /Script/Engine.MaterialInstanceDynamic))

(fn SpawnProyectile
  (params (DiferenciaAnguloSpawn :type Float%20%28double-precision%29))
  (bind _scene (Variables|Default|GetScene))
  (bind _returnvalue (Transformation|GetWorldRotation _scene))
  (Game|SpawnActorfromClass "/Game/Blueprints/BP_ProyectileBase.BP_ProyectileBase_C" (Math|Transform|MakeTransform (Transformation|GetActorLocation) (Math|Rotator|MakeRotator (.roll _returnvalue) (.pitch _returnvalue) (+ (.yaw _returnvalue) DiferenciaAnguloSpawn))) "AlwaysSpawn" "MultiplyWithRoot" 0 0))

(fn HandleSightSense
  (params (Actor :type Actor%20Object%20Reference) (Estimulo :type AI%20Stimulus%20Structure))
  (bind _returnvalue (Class|AIPerceptionSystem|GetSenseClassforStimulus Estimulo))
  (if (== _returnvalue "/Script/AIModule.AISense_Sight")
    (if true
      _
      (else
        (return))))
  (return))

(fn NewFunction)