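; BP_Spawner is an area spawner that populates a box volume with several enemy types when EscogerSalidas fires its LlamadaSpawners event.
; Per-type settings toggle and count each enemy (dogs, seeders, wheels, planters, statues, vacuums, oilers), each placed at a random point in the box.
; Seeders also get random yaw and a random SemilleroType.
; The construction script sizes the box from SpawnAreaSize.
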(event Custom|Spawn
  (bind _estatuas (Variables|Enemigos|Getestatuas))
  (bind _aspiradoras (Variables|Enemigos|GetAspiradoras))
  (bind _perros (Variables|Enemigos|GetPerros))
  (bind _semilleros (Variables|Enemigos|GetSemilleros))
  (bind _ruedas (Variables|Enemigos|GetRuedas))
  (bind _maceteros (Variables|Enemigos|GetMaceteros))
  (bind _aceitoso (Variables|Enemigos|GetAceitoso))
  (Utilities|FlowControl|Sequence
    (:then_0
      (if (.spawn? _perros)
        (for _index (range 1 (.numbertospawn _perros))
          (bind _location (CallFunction|GetRandomPointinArea))
          (Game|SpawnActorfromClass "/Game/Blueprints/Enemies/BP_Perro.BP_Perro_C" (Math|Transform|MakeTransform _location "0, 0, 0" "1.000000,1.000000,1.000000") "Undefined" "MultiplyWithRoot" 0 0))))
    (:then_1
      (if (.spawn? _semilleros)
        (for _index_2 (range 1 (.numbertospawn _semilleros))
          (bind _location_2 (CallFunction|GetRandomPointinArea))
          (bind _returnvalue (Game|SpawnActorfromClass "/Game/Blueprints/Enemies/BP_EnemySemillero.BP_EnemySemillero_C" (Math|Transform|MakeTransform _location_2 (Math|Rotator|MakeRotator 0.0 0.0 (.yaw (Math|Random|RandomRotator false))) "1.000000,1.000000,1.000000") "AdjustIfPossibleButAlwaysSpawn" "MultiplyWithRoot" 0 0))
          (Default|SetupType _returnvalue (.OutItem (Utilities|Array|Random (Variables|Default|GetSemilleroType)))))))
    (:then_2
      (if (.spawn? _ruedas)
        (for _index_3 (range 1 (.numbertospawn _ruedas))
          (bind _location_3 (CallFunction|GetRandomPointinArea))
          (Game|SpawnActorfromClass "/Game/Blueprints/Enemies/BP_Rueda.BP_Rueda_C" (Math|Transform|MakeTransform _location_3 "0, 0, 0" "1.000000,1.000000,1.000000") "AdjustIfPossibleButAlwaysSpawn" "MultiplyWithRoot" 0 0))))
    (:then_3
      (if (.spawn? _maceteros)
        (for _index_4 (range 1 (.numbertospawn _maceteros))
          (bind _location_4 (CallFunction|GetRandomPointinArea))
          (Game|SpawnActorfromClass "/Game/Blueprints/Enemies/BP_Maceta.BP_Maceta_C" (Math|Transform|MakeTransform _location_4 "0, 0, 0" "1.000000,1.000000,1.000000") "AdjustIfPossibleButAlwaysSpawn" "MultiplyWithRoot" 0 0))))
    (:then_4
      (if (.spawn? _estatuas)
        (for _index_5 (range 1 (.numbertospawn _estatuas))
          (bind _location_5 (CallFunction|GetRandomPointinArea))
          (Game|SpawnActorfromClass "/Game/Blueprints/BP_estatua.BP_estatua_C" (Math|Transform|MakeTransform _location_5 "0, 0, 0" "1.000000,1.000000,1.000000") "AdjustIfPossibleButAlwaysSpawn" "MultiplyWithRoot" 0 0))))
    (:then_5
      (if (.spawn? _aspiradoras)
        (for _index_6 (range 1 (.numbertospawn _aspiradoras))
          (bind _location_6 (CallFunction|GetRandomPointinArea))
          (Game|SpawnActorfromClass "/Game/Blueprints/Enemies/BP_EnemyAspiradora.BP_EnemyAspiradora_C" (Math|Transform|MakeTransform _location_6 "0, 0, 0" "1.000000,1.000000,1.000000") "AdjustIfPossibleButAlwaysSpawn" "MultiplyWithRoot" 0 0))))
    (:then_6
      (if (.spawn? _aceitoso)
        (for _index_7 (range 1 (.numbertospawn _aceitoso))
          (bind _location_7 (CallFunction|GetRandomPointinArea))
          (Game|SpawnActorfromClass "/Game/Blueprints/Enemies/BP_EnemyAceitador.BP_EnemyAceitador_C" (Math|Transform|MakeTransform _location_7 "0, 0, 0" "1.000000,1.000000,1.000000") "AdjustIfPossibleButAlwaysSpawn" "MultiplyWithRoot" 0 0))))))

(event EventBeginPlay
  (EventDispatchers|BindEventtoLlamadaSpawners (Variables|Default|GetescogerSalidas) (delegate Custom|Spawn)))

(fn ConstructionScript
  (Components|Box|SetBoxExtent (Variables|Default|GetSpawnArea) (Variables|Default|GetSpawn%20Area%20Size) true))

(fn GetRandomPointinArea
  (bind _spawnarea (Variables|Default|GetSpawnArea))
  (return (Math|Random|RandomPointinBoundingBox (Transformation|GetWorldLocation _spawnarea) (Components|Box|GetScaledBoxExtent _spawnarea))))