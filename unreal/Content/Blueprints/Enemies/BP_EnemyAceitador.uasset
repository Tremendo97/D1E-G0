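; Aceitador enemy that the player's pulse can stun, with state passed to its AI through Blackboard keys.
; On BeginPlay it binds to the player's Pulso dispatcher, setting "stunned" for a retriggerable duration when within pulse range.
; The dispara event plays a timeline that slides the Cabeza component vertically, then reverses it.
; Unconnected logic for the "visto" sighting flag and a fixed-length stun never runs, and stunnear is empty.
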(event Custom|stunnear)

(event Custom|dispara
  (Components|Timeline|SetPlayRate (Variables|Default|GetTimeline) (/ 1.0 0.7))
  (bind _newtrack_0 (Timeline|Timeline Play)
    (:Update
      (Transformation|SetRelativeLocation (Variables|Default|GetCabeza) (Math|Vector|Lerp(Vector) "0.000002,0.000000,-3.688122" "0.000002,0.000000,5.345986" _newtrack_0) false false))
    (:Finished
      (Timeline|Timeline Reverse))))

(event Custom|pulso
  (params (Tiempo :type Float%20%28double-precision%29) (Distancia :type Float%20%28double-precision%29))
  (if (<= (Math|Vector|Distance(Vector) (Transformation|GetActorLocation (Variables|Default|GetAs%20BP%20Personaje)) (Transformation|GetActorLocation)) Distancia)
    (AI|Components|Blackboard|SetValueasBool (AI|GetBlackboard (AI|GetAIController self)) (Utilities|Name|MakeLiteralName "stunned") true)
    (Utilities|FlowControl|RetriggerableDelay Tiempo)
    (AI|Components|Blackboard|SetValueasBool (AI|GetBlackboard (AI|GetAIController self)) (Utilities|Name|MakeLiteralName "stunned") false)))

(event EventBeginPlay
  (bind _asbp_personaje (Utilities|Casting|CastToBP_Personaje (Game|GetPlayerCharacter 0)))
  (EventDispatchers|BindEventtoPulso _asbp_personaje (delegate Custom|pulso))
  (Variables|Default|SetAs%20BP%20Personaje _asbp_personaje))

(fn ConstructionScript)