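; BP_stunner is an enemy helper that stuns the AI of its parent actor, presumably as a child actor attached to an enemy.
; Its stunn event sets the "stunned" key on the parent AI controller's blackboard to true, then clears it after a ten-second retriggerable delay.
; Calling stunn again during that window restarts the timer, extending the stun.
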(event Custom|stunn
  (AI|Components|Blackboard|SetValueasBool (AI|GetBlackboard (AI|GetAIController (Actor|GetParentActor))) (Utilities|Name|MakeLiteralName "stunned") true)
  (Utilities|FlowControl|RetriggerableDelay 1e+01)
  (AI|Components|Blackboard|SetValueasBool (AI|GetBlackboard (AI|GetAIController (Actor|GetParentActor))) (Utilities|Name|MakeLiteralName "stunned") false))

(event EventBeginPlay)

(event Collision|EventActorBeginOverlap
  (params (OtherActor :type Actor%20Object%20Reference)))

(event EventTick
  (params (DeltaSeconds :type Float%20%28single-precision%29)))

(fn ConstructionScript)