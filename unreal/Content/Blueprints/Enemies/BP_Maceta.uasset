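; BP_Maceta is an enemy Blueprint that switches its AI target to the squirrel (Ardilla) the player creates.
; On BeginPlay it binds to the player character's CrearArdilla event, then writes each new squirrel into the Blackboard "Target" key.
; It also binds to that squirrel's EndPlay, which sets "Target" back to the player if the Blackboard is still valid.
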(event Custom|On%20Crear%20Ardilla
  (params (Arilla%20Reference :type BP%20Ardilla%20Object%20Reference))
  ;[1 0.5616 0.3172] Ardilla
  (Game|BindEventtoOnEndPlay Arilla%20Reference (delegate Custom|On%20Ardilla%20Destroyed))
  (AI|Components|Blackboard|SetValueasObject (AI|GetBlackboard 0) (Utilities|Name|MakeLiteralName "Target") Arilla%20Reference))

(event Custom|On%20Ardilla%20Destroyed
  (params (Actor :type Actor%20Object%20Reference) (EndPlayReason :type EEndPlayReason%20Enum :default "Destroyed"))
  (bind _returnvalue (AI|GetBlackboard 0))
  ;[1 0.5616 0.3172] Ardilla
  (Game|UnbindEventfromOnEndPlay Actor (delegate Custom|On%20Ardilla%20Destroyed))
  (Utilities|IsValid _returnvalue
    (:Is%20Valid
      (AI|Components|Blackboard|SetValueasObject _returnvalue (Utilities|Name|MakeLiteralName "Target") (Game|GetPlayerCharacter 0)))))

(event EventBeginPlay
  (bind _asbp_personaje (Utilities|Casting|CastToBP_Personaje (Game|GetPlayerCharacter 0)))
  (EventDispatchers|BindEventtoCrearArdilla _asbp_personaje (delegate Custom|On%20Crear%20Ardilla)))

(fn ConstructionScript)