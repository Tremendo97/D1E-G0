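; BP_escogerSalidas is an actor that chooses exit locations at random when play begins.
; It picks two entries from the Salidas location array, spawns a half-scale BP_salidas at each, and removes each used entry to avoid repeating it.
; It then loops over all BP_Spawner actors with an empty body.
; A height check against Limite and a MirarBarcos call loop are left disconnected and never run.
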(event EventBeginPlay
  (for _index (range 0 1)
    (bind _output_get (Variables|Default|Setaleatorio (Math|Random|RandomIntegerinRange 0 (- (Utilities|Array|Length (Variables|Default|Getsalidas)) 1))))
    (Game|SpawnActorfromClass "/Game/Blueprints/BP_salidas.BP_salidas_C" (Math|Transform|MakeTransform (Utilities|Array|Get(acopy) (Variables|Default|Getsalidas) _output_get) "0, 0, 0" "0.500000,0.500000,0.500000") "Undefined" "MultiplyWithRoot" 0 0)
    (Utilities|Array|RemoveIndex (Variables|Default|Getsalidas) (Variables|Default|Getaleatorio)))
  (bind _outactors (Actor|GetAllActorsOfClass "/Game/Blueprints/Enemies/BP_Spawner.BP_Spawner_C"))
  (for _array_element _outactors
    _))

(fn ConstructionScript)