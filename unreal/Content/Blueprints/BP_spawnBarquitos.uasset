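; BP_spawnBarquitos is a boat spawner that follows the player along X, creating and removing BP_barquitos.
; Batches spawn at random points in the Spawn box on BeginPlay and player overlap with DetectPlayer, repeating after a delay while nearby.
; A global actor count caps spawning, and DoOnce caches a shared spawn height.
; The Despawn box destroys tagged boats; the construction script configures all three boxes from variables.
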(event OnComponentBeginOverlap(detectPlayer)
  (params (OverlappedComponent :type Primitive%20Component%20Object%20Reference) (OtherActor :type Actor%20Object%20Reference) (OtherComp :type Primitive%20Component%20Object%20Reference) (OtherBodyIndex :type Integer) (bFromSweep :type Boolean) (SweepResult :type Hit%20Result%20Structure%20%28by%20ref%29))
  (if (Actor|ActorHasTag OtherActor "Personaje")
    (Variables|Default|Setcerca true)
    (CallFunction|SpawnBarquitos)))

(event OnComponentEndOverlap(detectPlayer)
  (params (OverlappedComponent :type Primitive%20Component%20Object%20Reference) (OtherActor :type Actor%20Object%20Reference) (OtherComp :type Primitive%20Component%20Object%20Reference) (OtherBodyIndex :type Integer))
  (if (Actor|ActorHasTag OtherActor "Personaje")
    (Variables|Default|Setcerca false)))

(event OnComponentBeginOverlap(despawn)
  (params (OverlappedComponent :type Primitive%20Component%20Object%20Reference) (OtherActor :type Actor%20Object%20Reference) (OtherComp :type Primitive%20Component%20Object%20Reference) (OtherBodyIndex :type Integer) (bFromSweep :type Boolean) (SweepResult :type Hit%20Result%20Structure%20%28by%20ref%29))
  (if (Actor|ActorHasTag OtherActor "barquito")
    (Actor|DestroyActor OtherActor)))

(event Custom|spawn%20barquitos
  (bind _spawn (Variables|Default|Getspawn))
  (bind _returnvalue (Transformation|GetWorldLocation _spawn))
  (bind _returnvalue_2 (Components|Box|GetScaledBoxExtent _spawn))
  (bind _returnvalue_3 (Math|Random|RandomPointinBoundingBox _returnvalue _returnvalue_2))
  (for _index (range 0 (Variables|Default|Getbarcos)) :!label _label
    (Utilities|FlowControl|Sequence
      (:then_0
        (bind _outactors (Actor|GetAllActorsOfClass "/Game/Blueprints/BP_barquitos.BP_barquitos_C"))
        (if (> (Utilities|Array|Length _outactors) 10)
          _
          (else
            (Game|SpawnActorfromClass "/Game/Blueprints/BP_barquitos.BP_barquitos_C" (Math|Transform|MakeTransform (Math|Vector|MakeVector (.x _returnvalue_3) (.y _returnvalue_3) (stale _output_get)) "0, 0, 0" "1.000000,1.000000,1.000000") "Undefined" "MultiplyWithRoot" 0 0)))
        (if (== _index (Variables|Default|Getbarcos))
          (Utilities|FlowControl|Delay 1.0)
          (if (Variables|Default|Getcerca)
            (goto _label))))
      (:then_1
        (Utilities|FlowControl|DoOnce false
          (:Completed
            (bind _output_get (Variables|Default|SetReturn%20Value%20Z (.z _returnvalue_3)))))))))

(event EventTick
  (params (DeltaSeconds :type Float%20%28single-precision%29))
  (bind _returnvalue (Transformation|GetActorLocation))
  (Transformation|SetActorLocation (Math|Vector|MakeVector (.x (Transformation|GetActorLocation (Variables|Default|GetAs%20BP%20Personaje))) (.y _returnvalue) (.z _returnvalue)) false false))

(event EventBeginPlay
  (CallFunction|SpawnBarquitos)
  (bind _asbp_personaje (Utilities|Casting|CastToBP_Personaje (Game|GetPlayerCharacter 0)))
  (Variables|Default|SetAs%20BP%20Personaje _asbp_personaje))

(fn ConstructionScript
  (Components|Box|SetBoxExtent (Variables|Default|Getspawn) (Variables|Default|GetspawnExtent) true)
  (Components|Box|SetBoxExtent (Variables|Default|GetdetectPlayer) (Variables|Default|Getdetectar%20jugador) true)
  (Components|Box|SetBoxExtent (Variables|Default|Getdespawn) (Variables|Default|GetdespawnExtent) true)
  (Transformation|AddWorldOffset (Variables|Default|Getspawn) (Variables|Default|GetspawnLocation) false false)
  (Transformation|AddWorldOffset (Variables|Default|Getdespawn) (Variables|Default|GetdespawnLocation) false false))