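; BP_estatua is a statue actor that orients and grounds itself when placed in the level.
; Its construction script searches all BP_salidas actors for the closest, then sets yaw so forward X points away from it, keeping pitch and roll.
; A long downward Visibility trace then snaps it onto the surface below.
; In the event graph, MirarBarcos is empty and a similar orientation chain is left unconnected.
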(event Custom|MirarBarcos)

(fn ConstructionScript
  (bind _returnvalue (Transformation|GetActorLocation))
  (bind _returnvalue_2 (Transformation|GetActorRotation))
  (bind _outactors (Actor|GetAllActorsOfClass "/Game/Blueprints/BP_salidas.BP_salidas_C"))
  (for _array_element _outactors
    (Utilities|FlowControl|Sequence
      (:then_0
        (Utilities|FlowControl|DoOnce false
          (:Completed
            (Variables|Default|SetArray%20Element _array_element))))
      (:then_1
        (if (< (Transformation|GetDistanceTo _array_element self) (Transformation|GetDistanceTo (Variables|Default|GetArray%20Element) self))
          (Variables|Default|SetArray%20Element _array_element)))))
  (Transformation|SetActorRotation (Math|Rotator|MakeRotator (.roll _returnvalue_2) (.pitch _returnvalue_2) (.yaw (Math|Conversions|RotationFromXVector (- (Transformation|GetActorLocation) (Transformation|GetActorLocation (Variables|Default|GetArray%20Element)))))))
  (bind (_outhit _returnvalue_3) (Collision|LineTraceByChannel _returnvalue (- _returnvalue "0.000000,0.000000,1000000.000000") "TraceTypeQuery1" false 0 "None"))
  (if _returnvalue_3
    (Transformation|SetActorLocation (.Location (Collision|BreakHitResult _outhit)) false false)))