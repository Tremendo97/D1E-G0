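; Capturable antenna zone that the player dominates by staying inside its sphere, whose radius is set in the construction script.
; While the tagged character overlaps, the antenna spins and a delayed loop advances progress through the W_dominando widget.
; Completion spawns BP_Energia pickups at random reachable points, plays a Niagara effect and increments the player's Dominados count.
; Leaving early stops the spin and loop, re-arms the DoOnce and plays a widget animation after a retriggerable delay.
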(event OnComponentBeginOverlap(Sphere)
  (params (OverlappedComponent :type Primitive%20Component%20Object%20Reference) (OtherActor :type Actor%20Object%20Reference) (OtherComp :type Primitive%20Component%20Object%20Reference) (OtherBodyIndex :type Integer) (bFromSweep :type Boolean) (SweepResult :type Hit%20Result%20Structure%20%28by%20ref%29))
  (bind _sphere (Variables|Default|GetSphere))
  (bind _in_sphere_radius (Variables|Default|GetIn%20Sphere%20Radius))
  (bind _returnvalue (Transformation|GetWorldLocation _sphere))
  (bind _randomlocation (AI|Navigation|GetRandomReachablePointinRadius _returnvalue _in_sphere_radius 0 0))
  (bind (_x _y) (Math|Vector|BreakVector _randomlocation))
  (if (Components|ComponentHasTag OtherComp "Personaje")
    (CallFunction|RotarAntena)
    (Utilities|FlowControl|DoOnce false
      (:Completed
        (if (not (Variables|Default|Getactivado))
          (Utilities|IsValid (Variables|Default|GetNewVar_0)
            (:Is%20Valid
              (if (Variables|Default|Getoculta)
                (Default|PlayAnimation1 (Variables|Default|GetNewVar_0))))
            (:Is%20Not%20Valid
              (bind _returnvalue_2 (UserInterface|CreateWidget "/Game/UI/W_dominando.W_dominando_C"))
              (bind _output_get (Variables|Default|SetNewVar_0 _returnvalue_2))
              (UserInterface|Viewport|AddtoViewport _output_get 0)))
          (Variables|Default|Setseguir true)
          (bind _newparam (Default|Sumar _output_get :!label _label))
          (if (Variables|Default|Getseguir)
            (Utilities|FlowControl|Delay 0.1)
            (if (>= _newparam 1.0)
              (for _index (range 0 3)
                (Game|SpawnActorfromClass "/Game/Blueprints/BP_Energia.BP_Energia_C" (Math|Transform|MakeTransform (Math|Vector|MakeVector _x _y (.Z (Math|Vector|BreakVector _returnvalue))) "0, 0, 0" "1.000000,1.000000,1.000000") "Undefined" "MultiplyWithRoot" 0 0))
              (Default|PlayAnimation (Variables|Default|GetNewVar_0))
              (Variables|Default|Setactivado true)
              (Niagara|SpawnSystematLocation "/Game/Particles/NS_DominarZona.NS_DominarZona" (Transformation|GetWorldLocation (Variables|Default|GetANTENA)))
              (bind _asbp_personaje (Utilities|Casting|CastToBP_Personaje (Game|GetPlayerCharacter 0)))
              (Variables|/Game/Blueprints/BP_Personaje.BP_Personaje_C|Setdominados _asbp_personaje (+ (Variables|/Game/Blueprints/BP_Personaje.BP_Personaje_C|Getdominados _asbp_personaje) 1))
              (else
                (goto _label)))))))))

(event OnComponentEndOverlap(Sphere)
  (params (OverlappedComponent :type Primitive%20Component%20Object%20Reference) (OtherActor :type Actor%20Object%20Reference) (OtherComp :type Primitive%20Component%20Object%20Reference) (OtherBodyIndex :type Integer))
  (bind _sphere (Variables|Default|GetSphere))
  (bind _in_sphere_radius (Variables|Default|GetIn%20Sphere%20Radius))
  (bind _returnvalue (Transformation|GetWorldLocation _sphere))
  (bind _randomlocation (AI|Navigation|GetRandomReachablePointinRadius _returnvalue _in_sphere_radius 0 0))
  (bind (_x _y) (Math|Vector|BreakVector _randomlocation))
  (if (Components|ComponentHasTag OtherComp "Personaje")
    (if (not (Variables|Default|Getactivado))
      (CallFunction|Parar)
      (Utilities|FlowControl|Sequence
        (:then_0
          (Variables|Default|Setseguir false)
          (Utilities|FlowControl|RetriggerableDelay 5.0)
          (Default|PlayAnimation (Variables|Default|GetNewVar_0))
          (Variables|Default|Setoculta true))
        (:then_1
          (Utilities|FlowControl|DoOnce false) ; enters at Reset
        )))))

(event Custom|RotarAntena
  (bind _alfa (Timeline|Rotate Play)
    (:Update
      (Transformation|SetRelativeRotation (Variables|Default|GetANTENA) (Math|Rotator|Lerp(Rotator) "0, 0, 0" "0.000000,360.000000,0.000000" _alfa) false false))))

(event Custom|Parar
  (bind _alfa (Timeline|Rotate Stop)
    (:Update
      (Transformation|SetRelativeRotation (Variables|Default|GetANTENA) (Math|Rotator|Lerp(Rotator) "0, 0, 0" "0.000000,360.000000,0.000000" _alfa) false false))))

(fn ConstructionScript
  (Components|Sphere|SetSphereRadius (Variables|Default|GetSphere) (Variables|Default|GetIn%20Sphere%20Radius) true))