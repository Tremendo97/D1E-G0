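; BP_salto is a launch pad that throws the player when a "Player"-tagged component enters its Box.
; On overlap it zeroes the BP_Personaje's velocity, sets Stunned, and prints the launch vector.
; It launches player character 0 along the up vector rotated by Girox roll and Giroz yaw, scaled by Velocidad.
; The node that would clear Stunned is unconnected, so this actor never resets it.
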(event OnComponentBeginOverlap(Box)
  (params (OverlappedComponent :type Primitive%20Component%20Object%20Reference) (OtherActor :type Actor%20Object%20Reference) (OtherComp :type Primitive%20Component%20Object%20Reference) (OtherBodyIndex :type Integer) (bFromSweep :type Boolean) (SweepResult :type Hit%20Result%20Structure%20%28by%20ref%29))
  (bind _velocidad (Variables|Default|Getvelocidad))
  (bind _giroz (Variables|Default|Getgiroz))
  (bind _girox (Variables|Default|Getgirox))
  (bind _returnvalue (Math|Vector|RotateVector "0.000000,0.000000,1.000000" (Math|Rotator|MakeRotator _girox 0.0 _giroz)))
  (bind _returnvalue_2 (* _returnvalue _velocidad))
  (if (Components|ComponentHasTag OtherComp "Player")
    (bind _asbp_personaje (Utilities|Casting|CastToBP_Personaje OtherActor))
    (Variables|/Script/Engine.MovementComponent|SetVelocity (Variables|/Script/Engine.Character|GetCharacterMovement _asbp_personaje) "0, 0, 0")
    (Variables|/Game/Blueprints/BP_Personaje.BP_Personaje_C|SetStunned _asbp_personaje true)
    (Development|PrintString (Utilities|String|ToString(Vector) _returnvalue_2))
    (Character|LaunchCharacter (Game|GetPlayerCharacter 0) _returnvalue_2 false false)))

(event EventBeginPlay)

(event Collision|EventActorBeginOverlap
  (params (OtherActor :type Actor%20Object%20Reference)))

(event EventTick
  (params (DeltaSeconds :type Float%20%28single-precision%29)))

(fn ConstructionScript)