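; Player character with an orbiting ball (Bola), steered by mouse or gamepad at a variable radius.
; Delay loops rotate the ball with angular speed derived from tangential speed over radius, biased by vacuum actors that pull it.
; Traces toggle a "Gate" material parameter on walls occluding the camera.
; Projectile hits drain balance into a stun or ball energy into death, and it also handles pause and wheat foliage.
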(event OnComponentBeginOverlap(cilindro)
  (params (OverlappedComponent :type Primitive%20Component%20Object%20Reference) (OtherActor :type Actor%20Object%20Reference) (OtherComp :type Primitive%20Component%20Object%20Reference) (OtherBodyIndex :type Integer) (bFromSweep :type Boolean) (SweepResult :type Hit%20Result%20Structure%20%28by%20ref%29))
  ;[1 0.9435 0.3497 1 60] Pisar Trigo
  (bind _asinteractive_wheat_foliage (Utilities|Casting|CastToInteractiveWheatFoliage OtherComp))
  (Utilities|IsValid _asinteractive_wheat_foliage
    (:Is%20Valid
      (Default|EventHitFoliage _asinteractive_wheat_foliage SweepResult))))

(event OnComponentBeginOverlap(bola)
  (params (OverlappedComponent :type Primitive%20Component%20Object%20Reference) (OtherActor :type Actor%20Object%20Reference) (OtherComp :type Primitive%20Component%20Object%20Reference) (OtherBodyIndex :type Integer) (bFromSweep :type Boolean) (SweepResult :type Hit%20Result%20Structure%20%28by%20ref%29))
  ;[1 0.9435 0.3497 1 60] Pisar Trigo
  (bind _asinteractive_wheat_foliage (Utilities|Casting|CastToInteractiveWheatFoliage OtherComp))
  (Utilities|IsValid _asinteractive_wheat_foliage
    (:Is%20Valid
      (Default|EventHitFoliage _asinteractive_wheat_foliage SweepResult))))

(event Custom|Muerte
  (Variables|Default|Setmuerto true)
  (Utilities|FlowControl|Delay 1e+01)
  (Game|OpenLevel(byObjectReference) "/Game/Levels/L_Mainmenu.L_Mainmenu"))

(event Custom|Projectile%20Hit%20Bola
  ;[1 0.4882 0.4683 1 60] Hits Projectiles
  (bind _output_get (Variables|Default|Setenergia (- (Variables|Default|Getenergia) 1.0)))
  (if (== _output_get 0.0)
    (CallFunction|Muerte)
    (else
      (bind _output_get_2 (Variables|Default|SetenergiaProbabilidad (Math|Random|RandomIntegerinRange 0 10)))
      (if (== _output_get_2 8)
        (Utilities|FlowControl|DoOnce false :!label _label
          (:Completed
            (if (Variables|Default|GetSpawnEnergia)
              (bind _returnvalue (Game|SpawnActorfromClass "/Game/Blueprints/BP_Energia.BP_Energia_C" (Transformation|GetWorldTransform (Variables|Default|Getbola)) "Undefined" "MultiplyWithRoot" 0 0))
              (Default|CallCrearEnergia _returnvalue)
              (Variables|Default|SetenergiaProbabilidad 0)
              (goto _label Reset))))))))

(event Custom|noHayAspiradoras
  (params (NewParam :type Integer))
  (Variables|Default|Setaspiradoras false))

(event Custom|aspirar
  (bind _returnvalue (Transformation|GetActorTransform))
  (bind _bola (Variables|Default|Getbola))
  (bind _pos_aspiradoras (Variables|Default|Getpos_aspiradoras))
  (bind _returnvalue_2 (Transformation|GetActorLocation _pos_aspiradoras))
  (bind _relativelocation (Variables|/Script/Engine.SceneComponent|GetRelativeLocation _bola))
  (bind _returnvalue_3 (Math|Transform|InverseTransformLocation _returnvalue _returnvalue_2))
  (bind _returnvalue_4 (Math|Vector|Normalize (Math|Vector|MakeVector (.x _relativelocation) (.y _relativelocation) 0.0)))
  (if (Variables|Default|Getaspiradoras) :!label _label
    (Utilities|FlowControl|Delay 0.001)
    (Utilities|FlowControl|Sequence
      (:then_0
        (if (not (Variables|Default|Getrotando))
          (Variables|Default|Setseguir false)
          (Variables|Default|Setvelocidad%20de%20giro (Math|Interpolation|FInterptoConstant (Variables|Default|Getvelocidad%20de%20giro) (|(v/r) (Variables|Default|Getradio) (Variables|Default|Getvelocidad%20tangencial)) (Utilities|Time|GetWorldDeltaSeconds) 1e+06))
          (Transformation|SetRelativeLocation (Variables|Default|Getbola) (* (Math|Vector|RotateVector _returnvalue_4 (Class|KismetMathLibrary|RInterptoConstant "0, 0, 0" (Math|Rotator|CombineRotators (Class|KismetMathLibrary|NegateRotator (Math|Conversions|RotationFromXVector _returnvalue_4)) (Math|Conversions|RotationFromXVector (Math|Vector|Normalize (Math|Vector|MakeVector (.x _returnvalue_3) (.y _returnvalue_3) 0.0)))) (Utilities|Time|GetWorldDeltaSeconds) (Variables|Default|Getvelocidad%20de%20giro))) (Variables|Default|Getradio)) true false)))
      (:then_1
        (goto _label)))))

(event Custom|Projectile%20Hit%20Personaje
  ;[1 0.4882 0.4683 1 60] Hits Projectiles
  (if (Variables|Default|GetcanGetHit)
    (bind _result (Math|Float|DecrementFloat (Variables|Default|GetEquilibrio))
      (:%20%20
        (if (<= _result 0.0)
          (Variables|Default|SetStunned true)
          (Variables|Default|SetcanGetHit false)
          (Rendering|Material|SetScalarParameterValue "/Game/Materials/Personaje/MPC_Personaje.MPC_Personaje" "Opacity" 0.3 :!class /Script/Engine.KismetMaterialLibrary)
          (Utilities|FlowControl|Delay 2.0)
          (Variables|Default|SetStunned false)
          (Variables|Default|SetEquilibrio 5.0)
          (Utilities|FlowControl|Delay 2.0)
          (Variables|Default|SetcanGetHit true)
          (Rendering|Material|SetScalarParameterValue "/Game/Materials/Personaje/MPC_Personaje.MPC_Personaje" "Opacity" 1.0 :!class /Script/Engine.KismetMaterialLibrary))))))

(event Custom|Check%20Paredes
  (bind _cilindro (Variables|Default|Getcilindro))
  (bind _returnvalue (Transformation|GetWorldLocation _cilindro))
  ;[0.4943 1 0.7271 1 60] Wall Opacity Mask
  (bind (_outhit _returnvalue_2) (Collision|LineTraceByChannel _returnvalue (+ "0.000000,0.000000,-5000.000000" _returnvalue) "TraceTypeQuery1" false 0 "None"))
  (if _returnvalue_2
    (if (not (Actor|ActorHasTag (.HitActor (Collision|BreakHitResult _outhit)) "City"))
      (Utilities|FlowControl|DoOnce false
        (:Completed
          (bind _outhits (Class|KismetSystemLibrary|CapsuleTraceMulti (Transformation|GetWorldLocation (Variables|Default|GetCamera)) (Transformation|GetWorldLocation (Variables|Default|Getcilindro)) 3e+01 0.0 "TraceTypeQuery3" false 0 "None" true))
          (for _array_element _outhits
            (Utilities|Array|AddUnique (Variables|Default|GetWallsToHide) (.HitActor (Collision|BreakHitResult _array_element))))
          (for _array_element_2 (Variables|Default|GetHiddenWalls)
            (if (not (Utilities|Array|ContainsItem (Variables|Default|GetWallsToHide) _array_element_2))
              (bind _asstatic_mesh_actor (Utilities|Casting|CastToStaticMeshActor _array_element_2))
              (Rendering|Material|SetScalarParameterValueonMaterials (Variables|/Script/Engine.StaticMeshActor|GetStaticMeshComponent _asstatic_mesh_actor) "Gate" 0.0)
              (Utilities|Array|RemoveItem (Variables|Default|GetHiddenWalls) _array_element_2)))
          (for _array_element_3 (Variables|Default|GetWallsToHide)
            (if (not (Utilities|Array|ContainsItem (Variables|Default|GetHiddenWalls) _array_element_3))
              (Utilities|Array|AddUnique (Variables|Default|GetHiddenWalls) _array_element_3)
              (bind _asstatic_mesh_actor_2 (Utilities|Casting|CastToStaticMeshActor _array_element_3))
              (Rendering|Material|SetScalarParameterValueonMaterials (Variables|/Script/Engine.StaticMeshActor|GetStaticMeshComponent _asstatic_mesh_actor_2) "Gate" 1.0)))
          (CallFunction|ResetCheckWalls)
          (Utilities|Array|Clear (Variables|Default|GetWallsToHide)))))))

(event Custom|ResetCheckWalls
  ;[0.4943 1 0.7271 1 60] Wall Opacity Mask
  (Utilities|FlowControl|DoOnce false) ; enters at Reset
)

(event Input|EnhancedActionEvents|EnhancedInputActionIA_myMove
  (params (ActionValue :type Vector%202D%20Structure) (ElapsedSeconds :type Float%20%28double-precision%29) (TriggeredSeconds :type Float%20%28double-precision%29) (InputAction :type Input%20Action%20Object%20Reference :default "/Game/Blueprints/Inputs/IA_myMove.IA_myMove"))
  (bind _returnvalue (Transformation|GetActorRotation))
  (bind _returnvalue_2 (Transformation|GetActorRotation))
  (bind _charactermovement (Variables|Character|GetCharacterMovement))
  (bind _base_velocity (Variables|Default|GetBase%20Velocity))
  (bind _mesh (Variables|Character|GetMesh))
  (bind _relativerotation (Variables|/Script/Engine.SceneComponent|GetRelativeRotation _mesh))
  (if (not (Variables|Default|Getmuerto))
    (if (> (Math|Vector|VectorLength (Math|Vector|MakeVector (.x ActionValue) (.y ActionValue) 0.0)) 0.2)
      (Transformation|SetRelativeRotation _mesh (Math|Rotator|MakeRotator (.roll _relativerotation) (.pitch _relativerotation) (.yaw (Math|Conversions|RotationFromXVector (Math|Vector|MakeVector (- 0.0 (.y ActionValue)) (- 0.0 (.x ActionValue)) 0.0)))) false false)
      (if (not (Variables|Default|GetStunned))
        (if (> (Math|Float|Absolute(Float) (.x ActionValue)) (Math|Float|Absolute(Float) (.y ActionValue)))
          (Variables|/Script/Engine.CharacterMovementComponent|SetMaxWalkSpeed _charactermovement (Math|Float|Absolute(Float) (* (.x ActionValue) _base_velocity)))
          (else
            (Variables|/Script/Engine.CharacterMovementComponent|SetMaxWalkSpeed _charactermovement (Math|Float|Absolute(Float) (* (.y ActionValue) _base_velocity)))))
        (Pawn|Input|AddMovementInput (Math|Vector|GetRightVector (Math|Rotator|MakeRotator (.roll _returnvalue) 0.0 (.yaw _returnvalue))) (.x ActionValue) false)
        (Pawn|Input|AddMovementInput (Math|Vector|GetForwardVector (Math|Rotator|MakeRotator 0.0 (.pitch _returnvalue_2) (.yaw _returnvalue_2))) (.y ActionValue) false)))))

(event Input|EnhancedActionEvents|EnhancedInputActionIA_rotacionEsferaraton
  (params (ActionValue :type Vector%202D%20Structure) (ElapsedSeconds :type Float%20%28double-precision%29) (TriggeredSeconds :type Float%20%28double-precision%29) (InputAction :type Input%20Action%20Object%20Reference :default "/Game/Blueprints/Inputs/IA_rotacionEsferaraton.IA_rotacionEsferaraton"))
  (bind _returnvalue (Transformation|GetActorTransform))
  (bind _returnvalue_2 (Game|GetPlayerController 0))
  (bind _returnvalue_3 (Game|GetPlayerController 0))
  (bind _bola (Variables|Default|Getbola))
  (bind _bola_2 (Variables|Default|Getbola))
  (bind _bola_3 (Variables|Default|Getbola))
  (bind _pos_aspiradoras (Variables|Default|Getpos_aspiradoras))
  (bind _returnvalue_4 (Transformation|GetActorLocation _pos_aspiradoras))
  (bind (_locationx _locationy) (Game|Player|GetMousePosition _returnvalue_2))
  (bind (_sizex _sizey) (HUD|GetViewportSize _returnvalue_2))
  (bind (_locationx_2 _locationy_2) (Game|Player|GetMousePosition _returnvalue_3))
  (bind (_sizex_2 _sizey_2) (HUD|GetViewportSize _returnvalue_3))
  (bind _relativelocation (Variables|/Script/Engine.SceneComponent|GetRelativeLocation _bola))
  (bind _relativelocation_2 (Variables|/Script/Engine.SceneComponent|GetRelativeLocation _bola_2))
  (bind _relativelocation_3 (Variables|/Script/Engine.SceneComponent|GetRelativeLocation _bola_3))
  (bind _returnvalue_5 (Math|Transform|InverseTransformLocation _returnvalue _returnvalue_4))
  (bind _returnvalue_6 (Math|Vector|Normalize (Math|Vector|MakeVector (.x _relativelocation_2) (.y _relativelocation_2) 0.0)))
  (bind _returnvalue_7 (* _sizey 0.5))
  (bind _returnvalue_8 (* _sizex 0.5))
  (bind _returnvalue_9 (- _locationy _returnvalue_7))
  (bind _returnvalue_10 (- _locationx _returnvalue_8))
  (bind _returnvalue_11 (- 0.0 _returnvalue_9))
  (bind _returnvalue_12 (Math|Vector|Normalize (Math|Vector|MakeVector _returnvalue_11 _returnvalue_10 0.0)))
  (bind _returnvalue_13 (Math|Vector|CrossProduct (Math|Vector|MakeVector (.x _returnvalue_12) (.y _returnvalue_12) 0.0) (Math|Vector|MakeVector (.x _relativelocation) (.y _relativelocation) 0.0)))
  (bind _returnvalue_14 (> (.z _returnvalue_13) 0.0))
  (:Triggered
    (if (not (Variables|Default|Getmuerto))
      (Variables|Default|Setrotando true)
      (Variables|Default|Setseguir true)
      (if (Variables|Default|Getseguir) :!label _label
        (Utilities|FlowControl|Delay 0.001)
        (Utilities|FlowControl|Sequence
          (:then_0
            (if (Variables|Default|Getaspiradoras)
              (if (> (.z (Math|Vector|CrossProduct (Math|Vector|MakeVector (.x _returnvalue_5) (.y _returnvalue_5) 0.0) (Math|Vector|MakeVector (.x _relativelocation_3) (.y _relativelocation_3) 0.0))) 0.0)
                (if _returnvalue_14
                  (Variables|Default|Setvelocidad%20de%20giro (Math|Interpolation|FInterptoConstant (Variables|Default|Getvelocidad%20de%20giro) 6e+02 (Utilities|Time|GetWorldDeltaSeconds) 1e+04))
                  (else
                    (Variables|Default|Setvelocidad%20de%20giro (Math|Interpolation|FInterptoConstant (Variables|Default|Getvelocidad%20de%20giro) 3e+01 (Utilities|Time|GetWorldDeltaSeconds) 1e+04))))
                (elif _returnvalue_14
                  (Variables|Default|Setvelocidad%20de%20giro (Math|Interpolation|FInterptoConstant (Variables|Default|Getvelocidad%20de%20giro) 3e+01 (Utilities|Time|GetWorldDeltaSeconds) 1e+04))
                  (else
                    (Variables|Default|Setvelocidad%20de%20giro (Math|Interpolation|FInterptoConstant (Variables|Default|Getvelocidad%20de%20giro) 6e+02 (Utilities|Time|GetWorldDeltaSeconds) 1e+04)))))
              (else
                (Variables|Default|Setvelocidad%20de%20giro (|(v/r) (Variables|Default|Getradio) (Variables|Default|Getvelocidad%20tangencial)))))
            (if (< (.z (Math|Vector|CrossProduct (Variables|/Script/Engine.SceneComponent|GetRelativeLocation (Variables|Default|Getbola)) (- (* (Math|Vector|RotateVector _returnvalue_6 (Class|KismetMathLibrary|RInterptoConstant "0, 0, 0" (Math|Rotator|CombineRotators (Class|KismetMathLibrary|NegateRotator (Math|Conversions|RotationFromXVector _returnvalue_6)) (Math|Conversions|RotationFromXVector (Math|Vector|Normalize (Math|Vector|MakeVector (- 0.0 (- _locationy_2 (* _sizey_2 0.5))) (- _locationx_2 (* _sizex_2 0.5)) 0.0)))) (Utilities|Time|GetWorldDeltaSeconds) (Variables|Default|Getvelocidad%20de%20giro))) (Variables|Default|Getradio)) "0.000000,0.000000,10.000000"))) 0.0)
              (Development|PrintString "izquierda")
              (if (Variables|Default|Getgiro_izquierda)
                (Variables|Default|Setgiro_derecha true)
                (Transformation|SetRelativeLocation (Variables|Default|Getbola) (- (* (Math|Vector|RotateVector _returnvalue_6 (Class|KismetMathLibrary|RInterptoConstant "0, 0, 0" (Math|Rotator|CombineRotators (Class|KismetMathLibrary|NegateRotator (Math|Conversions|RotationFromXVector _returnvalue_6)) (Math|Conversions|RotationFromXVector (Math|Vector|Normalize (Math|Vector|MakeVector (- 0.0 (- _locationy_2 (* _sizey_2 0.5))) (- _locationx_2 (* _sizex_2 0.5)) 0.0)))) (Utilities|Time|GetWorldDeltaSeconds) (Variables|Default|Getvelocidad%20de%20giro))) (Variables|Default|Getradio)) "0.000000,0.000000,10.000000") true false :!label _label_2)
                (if (Utilities|Operators|EqualEqual (- (* (Math|Vector|RotateVector _returnvalue_6 (Class|KismetMathLibrary|RInterptoConstant "0, 0, 0" (Math|Rotator|CombineRotators (Class|KismetMathLibrary|NegateRotator (Math|Conversions|RotationFromXVector _returnvalue_6)) (Math|Conversions|RotationFromXVector (Math|Vector|Normalize (Math|Vector|MakeVector (- 0.0 (- _locationy_2 (* _sizey_2 0.5))) (- _locationx_2 (* _sizex_2 0.5)) 0.0)))) (Utilities|Time|GetWorldDeltaSeconds) (Variables|Default|Getvelocidad%20de%20giro))) (Variables|Default|Getradio)) "0.000000,0.000000,10.000000") (Variables|/Script/Engine.SceneComponent|GetRelativeLocation (Variables|Default|Getbola)) 0.1)
                  (Variables|Default|Setseguir false)))
              (else
                (Development|PrintString "derecha")
                (if (Variables|Default|Getgiro_derecha)
                  (Variables|Default|Setgiro_izquierda true)
                  (goto _label_2)))))
          (:then_1
            (goto _label))))))
  (:Completed
    (Variables|Default|Setrotando false)))

(event Input|EnhancedActionEvents|EnhancedInputActionIA_rotacionEsferaMando
  (params (ActionValue :type Vector%202D%20Structure) (ElapsedSeconds :type Float%20%28double-precision%29) (TriggeredSeconds :type Float%20%28double-precision%29) (InputAction :type Input%20Action%20Object%20Reference :default "/Game/Blueprints/Inputs/IA_rotacionEsferaMando.IA_rotacionEsferaMando"))
  (bind _returnvalue (Transformation|GetActorTransform))
  (bind _returnvalue_2 (Math|Vector|Distance2D(Vector) :V1 (Math|Vector2D|MakeVector2D (.x ActionValue) (.y ActionValue))))
  (bind _bola (Variables|Default|Getbola))
  (bind _pos_aspiradoras (Variables|Default|Getpos_aspiradoras))
  (bind _bola_2 (Variables|Default|Getbola))
  (bind _bola_3 (Variables|Default|Getbola))
  (bind _radio_menor (Variables|Default|Getradio%20menor))
  (bind _returnvalue_3 (Transformation|GetActorLocation _pos_aspiradoras))
  (bind _relativelocation (Variables|/Script/Engine.SceneComponent|GetRelativeLocation _bola))
  (bind _relativelocation_2 (Variables|/Script/Engine.SceneComponent|GetRelativeLocation _bola_2))
  (bind _relativelocation_3 (Variables|/Script/Engine.SceneComponent|GetRelativeLocation _bola_3))
  (bind _returnvalue_4 (Math|Transform|InverseTransformLocation _returnvalue _returnvalue_3))
  (bind _returnvalue_5 (Math|Vector|Normalize (Math|Vector|MakeVector (.x _relativelocation_3) (.y _relativelocation_3) 0.0)))
  (if (not (Variables|Default|Getmuerto))
    (if (> _returnvalue_2 0.3)
      (Variables|Default|Setrotando true)
      (Variables|Default|Setseguir true)
      (Variables|Default|Setdireccion_x (* (/ (.x ActionValue) _returnvalue_2) _radio_menor))
      (Variables|Default|Setdireccion_y (* (/ (.y ActionValue) _returnvalue_2) _radio_menor))
      (if (Variables|Default|Getaspiradoras)
        (if (== (> (.z (Math|Vector|CrossProduct (Math|Vector|MakeVector (.x _returnvalue_4) (.y _returnvalue_4) 0.0) (Math|Vector|MakeVector (.x _relativelocation_2) (.y _relativelocation_2) 0.0))) 0.0) (> (.z (Math|Vector|CrossProduct (Math|Vector|MakeVector (Variables|Default|Getdireccion_x) (Variables|Default|Getdireccion_y) 0.0) (Math|Vector|MakeVector (.x _relativelocation) (.y _relativelocation) 0.0))) 0.0))
          (Variables|Default|Setvelocidad%20de%20giro 6e+02)
          (else
            (Variables|Default|Setvelocidad%20de%20giro 3e+01)))
        (else
          (Variables|Default|Setvelocidad%20de%20giro (/ (Variables|Default|Getvelocidad%20tangencial) (Variables|Default|Getradio)))))
      (if (Variables|Default|Getseguir) :!label _label
        (Utilities|FlowControl|Sequence
          (:then_0
            (Transformation|SetRelativeLocation (Variables|Default|Getbola) (- (* (Math|Vector|RotateVector _returnvalue_5 (Class|KismetMathLibrary|RInterptoConstant "0, 0, 0" (Math|Rotator|CombineRotators (Class|KismetMathLibrary|NegateRotator (Math|Conversions|RotationFromXVector _returnvalue_5)) (Math|Conversions|RotationFromXVector (Math|Vector|Normalize (Math|Vector|MakeVector (Variables|Default|Getdireccion_x) (Variables|Default|Getdireccion_y) 0.0)))) (Utilities|Time|GetWorldDeltaSeconds) (Variables|Default|Getvelocidad%20de%20giro))) (Variables|Default|Getradio)) "0.000000,0.000000,10.000000") true false)
            (if (Utilities|Operators|EqualEqual (- (* (Math|Vector|RotateVector _returnvalue_5 (Class|KismetMathLibrary|RInterptoConstant "0, 0, 0" (Math|Rotator|CombineRotators (Class|KismetMathLibrary|NegateRotator (Math|Conversions|RotationFromXVector _returnvalue_5)) (Math|Conversions|RotationFromXVector (Math|Vector|Normalize (Math|Vector|MakeVector (Variables|Default|Getdireccion_x) (Variables|Default|Getdireccion_y) 0.0)))) (Utilities|Time|GetWorldDeltaSeconds) (Variables|Default|Getvelocidad%20de%20giro))) (Variables|Default|Getradio)) "0.000000,0.000000,10.000000") (Variables|/Script/Engine.SceneComponent|GetRelativeLocation (Variables|Default|Getbola)) 0.1)
              (Variables|Default|Setseguir false)))
          (:then_1
            (Utilities|FlowControl|Delay 0.001)
            (goto _label))))
      (else
        (Variables|Default|Setrotando false)))))

(event Input|EnhancedActionEvents|EnhancedInputActionIA_cambioRadioMando
  (params (ActionValue :type Boolean) (ElapsedSeconds :type Float%20%28double-precision%29) (TriggeredSeconds :type Float%20%28double-precision%29) (InputAction :type Input%20Action%20Object%20Reference :default "/Game/Blueprints/Inputs/IA_cambioRadioMando.IA_cambioRadioMando"))
  (bind _radio_menor (Variables|Default|Getradio%20menor))
  (bind _bola (Variables|Default|Getbola))
  (bind _relativelocation (Variables|/Script/Engine.SceneComponent|GetRelativeLocation _bola))
  (bind _returnvalue (Math|Vector|Normalize (Math|Vector|MakeVector (.x _relativelocation) (.y _relativelocation) 0.0)))
  (:Triggered
    (if (not (Variables|Default|Getmuerto))
      (Utilities|FlowControl|Delay 0.01)
      (bind _output_get (Variables|Default|Setradio (Math|Interpolation|FInterptoConstant (Variables|Default|Getradio) (Variables|Default|Getradio%20mayor) (Utilities|Time|GetWorldDeltaSeconds) 5e+02)))
      (Variables|Default|Setvelocidad%20de%20giro (|(v/r) _output_get (Variables|Default|Getvelocidad%20tangencial)))
      (Transformation|SetRelativeLocation (Variables|Default|Getbola) (- (* (Math|Vector|RotateVector _returnvalue (Class|KismetMathLibrary|RInterptoConstant "0, 0, 0" (Math|Rotator|CombineRotators (Class|KismetMathLibrary|NegateRotator (Math|Conversions|RotationFromXVector _returnvalue)) (Math|Conversions|RotationFromXVector (Math|Vector|Normalize (Math|Vector|MakeVector (Variables|Default|Getdireccion_x) (Variables|Default|Getdireccion_y) 0.0)))) (Utilities|Time|GetWorldDeltaSeconds) (Variables|Default|Getvelocidad%20de%20giro))) (Variables|Default|Getradio)) "0.000000,0.000000,10.000000") true false :!label _label)
      (if (Utilities|Operators|EqualEqual (- (* (Math|Vector|RotateVector _returnvalue (Class|KismetMathLibrary|RInterptoConstant "0, 0, 0" (Math|Rotator|CombineRotators (Class|KismetMathLibrary|NegateRotator (Math|Conversions|RotationFromXVector _returnvalue)) (Math|Conversions|RotationFromXVector (Math|Vector|Normalize (Math|Vector|MakeVector (Variables|Default|Getdireccion_x) (Variables|Default|Getdireccion_y) 0.0)))) (Utilities|Time|GetWorldDeltaSeconds) (Variables|Default|Getvelocidad%20de%20giro))) (Variables|Default|Getradio)) "0.000000,0.000000,10.000000") (Variables|/Script/Engine.SceneComponent|GetRelativeLocation (Variables|Default|Getbola)) 0.1)
        (Variables|Default|Setseguir false))))
  (:Completed
    (if (!= (Variables|Default|Getradio) _radio_menor) :!label _label_2
      (if (not ActionValue)
        (Utilities|FlowControl|Delay 0.01)
        (Utilities|FlowControl|Sequence
          (:then_0
            (bind _output_get_2 (Variables|Default|Setradio (Math|Interpolation|FInterptoConstant (Variables|Default|Getradio) _radio_menor (Utilities|Time|GetWorldDeltaSeconds) 5e+02)))
            (Variables|Default|Setvelocidad%20de%20giro (|(v/r) _output_get_2 (Variables|Default|Getvelocidad%20tangencial)))
            (goto _label))
          (:then_1
            (goto _label_2)))))))

(event Input|EnhancedActionEvents|EnhancedInputActionIA_cambioRadioRaton
  (params (ActionValue :type Boolean) (ElapsedSeconds :type Float%20%28double-precision%29) (TriggeredSeconds :type Float%20%28double-precision%29) (InputAction :type Input%20Action%20Object%20Reference :default "/Game/Blueprints/Inputs/IA_cambioRadioRaton.IA_cambioRadioRaton"))
  (bind _returnvalue (Game|GetPlayerController 0))
  (bind _bola (Variables|Default|Getbola))
  (bind _radio_menor (Variables|Default|Getradio%20menor))
  (bind (_locationx _locationy) (Game|Player|GetMousePosition _returnvalue))
  (bind (_sizex _sizey) (HUD|GetViewportSize _returnvalue))
  (bind _relativelocation (Variables|/Script/Engine.SceneComponent|GetRelativeLocation _bola))
  (bind _returnvalue_2 (Math|Vector|Normalize (Math|Vector|MakeVector (.x _relativelocation) (.y _relativelocation) 0.0)))
  (:Triggered
    (if (not (Variables|Default|Getmuerto))
      (Utilities|FlowControl|Delay 0.01)
      (bind _output_get (Variables|Default|Setradio (Math|Interpolation|FInterptoConstant (Variables|Default|Getradio) (Variables|Default|Getradio%20mayor) (Utilities|Time|GetWorldDeltaSeconds) 5e+02)))
      (if (< (.z (Math|Vector|CrossProduct (Variables|/Script/Engine.SceneComponent|GetRelativeLocation (Variables|Default|Getbola)) (- (* (Math|Vector|RotateVector _returnvalue_2 (Class|KismetMathLibrary|RInterptoConstant "0, 0, 0" (Math|Rotator|CombineRotators (Class|KismetMathLibrary|NegateRotator (Math|Conversions|RotationFromXVector _returnvalue_2)) (Math|Conversions|RotationFromXVector (Math|Vector|Normalize (Math|Vector|MakeVector (- 0.0 (- _locationy (* _sizey 0.5))) (- _locationx (* _sizex 0.5)) 0.0)))) (Utilities|Time|GetWorldDeltaSeconds) (Variables|Default|Getvelocidad%20de%20giro))) (Variables|Default|Getradio)) "0.000000,0.000000,10.000000"))) 0.0) :!label _label
        (Development|PrintString "izquierda")
        (if (Variables|Default|Getgiro_izquierda)
          (Variables|Default|Setgiro_derecha true)
          (Transformation|SetRelativeLocation (Variables|Default|Getbola) (- (* (Math|Vector|RotateVector _returnvalue_2 (Class|KismetMathLibrary|RInterptoConstant "0, 0, 0" (Math|Rotator|CombineRotators (Class|KismetMathLibrary|NegateRotator (Math|Conversions|RotationFromXVector _returnvalue_2)) (Math|Conversions|RotationFromXVector (Math|Vector|Normalize (Math|Vector|MakeVector (- 0.0 (- _locationy (* _sizey 0.5))) (- _locationx (* _sizex 0.5)) 0.0)))) (Utilities|Time|GetWorldDeltaSeconds) (Variables|Default|Getvelocidad%20de%20giro))) (Variables|Default|Getradio)) "0.000000,0.000000,10.000000") true false :!label _label_2)
          (if (Utilities|Operators|EqualEqual (- (* (Math|Vector|RotateVector _returnvalue_2 (Class|KismetMathLibrary|RInterptoConstant "0, 0, 0" (Math|Rotator|CombineRotators (Class|KismetMathLibrary|NegateRotator (Math|Conversions|RotationFromXVector _returnvalue_2)) (Math|Conversions|RotationFromXVector (Math|Vector|Normalize (Math|Vector|MakeVector (- 0.0 (- _locationy (* _sizey 0.5))) (- _locationx (* _sizex 0.5)) 0.0)))) (Utilities|Time|GetWorldDeltaSeconds) (Variables|Default|Getvelocidad%20de%20giro))) (Variables|Default|Getradio)) "0.000000,0.000000,10.000000") (Variables|/Script/Engine.SceneComponent|GetRelativeLocation (Variables|Default|Getbola)) 0.1)
            (Variables|Default|Setseguir false)))
        (else
          (Development|PrintString "derecha")
          (if (Variables|Default|Getgiro_derecha)
            (Variables|Default|Setgiro_izquierda true)
            (goto _label_2))))))
  (:Completed
    (if (!= (Variables|Default|Getradio) _radio_menor) :!label _label_3
      (if (not ActionValue)
        (Utilities|FlowControl|Delay 0.01)
        (Utilities|FlowControl|Sequence
          (:then_0
            (bind _output_get_2 (Variables|Default|Setradio (Math|Interpolation|FInterptoConstant (Variables|Default|Getradio) _radio_menor (Utilities|Time|GetWorldDeltaSeconds) 5e+02)))
            (goto _label))
          (:then_1
            (goto _label_3)))))))

(event Input|EnhancedActionEvents|EnhancedInputActionIA_Pausa
  (params (ActionValue :type Boolean) (ElapsedSeconds :type Float%20%28double-precision%29) (TriggeredSeconds :type Float%20%28double-precision%29) (InputAction :type Input%20Action%20Object%20Reference :default "/Game/Blueprints/Inputs/IA_Pausa.IA_Pausa"))
  (bind _returnvalue (Game|GetPlayerController 0))
  (bind _returnvalue_2 (Game|GetPlayerController 0))
  ;[1 1 1 1 60] Pause Menu
  (:Started
    (if (Game|IsGamePaused)
      (Game|SetGamePaused false)
      (Widget|RemovefromParent (Variables|Default|GetPauseMenuWidget))
      (Game|SetGamePaused false)
      (Input|SetInputModeGameOnly _returnvalue_2 false)
      (Variables|/Script/Engine.PlayerController|SetbShowMouseCursor _returnvalue_2 false)
      (else
        (bind _returnvalue_3 (UserInterface|CreateWidget "/Game/UI/W_Pausemenu.W_Pausemenu_C" _returnvalue))
        (bind _output_get (Variables|Default|SetPauseMenuWidget _returnvalue_3))
        (UserInterface|Viewport|AddtoViewport _output_get 0)
        (Input|SetInputModeGameandUI _returnvalue (Variables|Default|GetPauseMenuWidget) "DoNotLock" true false)
        (Variables|/Script/Engine.PlayerController|SetbShowMouseCursor (Game|GetPlayerController 0) true)
        (Game|SetGamePaused true)))))

(event EventTick
  (params (DeltaSeconds :type Float%20%28single-precision%29))
  ;[1 1 1 1 60] Event Tick
  (CallFunction|CheckParedes)
  (if (== 0.0 (Math|Vector|VectorLength (Variables|/Script/Engine.MovementComponent|GetVelocity (Variables|Character|GetCharacterMovement))))
    (CallFunction|Parado)))

(event EventBeginPlay
  ;[1 1 1 1 60] BeginPlay
  (Physics|SetSimulatePhysics (Variables|Collision|GetCapsuleComponent) false)
  ;;[1 1 1] Camera Setup
  (bind _returnvalue (AddComponent|AddPostProcessComponent false))
  (Utilities|Struct|SetmembersinPostProcessSettings (Variables|/Script/Engine.PostProcessComponent|GetSettings _returnvalue) 0.4 144.0 (Variables|/Script/Engine.SpringArmComponent|GetTargetArmLength (Variables|Default|GetSpringArm1)))
  ;;[1 1 1] Controller Setup
  (bind _asplayer_controller (Utilities|Casting|CastToPlayerController (Pawn|GetController)))
  (Utilities|IsValid (PlayerController|LocalPlayerSubsystems|GetEnhancedInputLocalPlayerSubsystem _asplayer_controller)
    (:Is%20Valid
      (Input|AddMappingContext (PlayerController|LocalPlayerSubsystems|GetEnhancedInputLocalPlayerSubsystem _asplayer_controller) "/Game/Blueprints/Inputs/controlador_mando.controlador_mando" 0 "(bIgnoreAllPressedKeysUntilRelease=True,bForceImmediately=False,bNotifyUserSettings=False)"))))

(fn ConstructionScript)

(fn HayAspiradora
  (params (NewParam :type Actor%20Object%20Reference))
  (Variables|Default|Setpos_aspiradoras NewParam)
  (Variables|Default|Setaspiradoras true)
  (CallFunction|Aspirar)
  (return 0))

(fn Parado
  (bind _returnvalue (Collision|LineTraceByChannel (Transformation|GetActorLocation) (Math|Transform|TransformLocation (Transformation|GetActorTransform) (Math|Vector|RotateVector (Variables|/Script/Engine.SceneComponent|GetRelativeLocation (Variables|Default|Getbola)) "0.000000,15.000000,0.000000")) "TraceTypeQuery1" false 0 "ForOneFrame"))
  (if _returnvalue
    (Variables|Default|Setgiro_derecha false)
    (Variables|Default|Setgiro_izquierda true))
  (bind _returnvalue_2 (Collision|LineTraceByChannel (Transformation|GetActorLocation) (Math|Transform|TransformLocation (Transformation|GetActorTransform) (Math|Vector|RotateVector (Variables|/Script/Engine.SceneComponent|GetRelativeLocation (Variables|Default|Getbola)) "0.000000,-15.000000,0.000000")) "TraceTypeQuery1" false 0 "ForOneFrame"))
  (if _returnvalue_2
    (Variables|Default|Setgiro_derecha true)
    (Variables|Default|Setgiro_izquierda false)))