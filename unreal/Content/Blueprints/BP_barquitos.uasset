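; BP_barquitos is an actor, by its name a small boat, that runs a sailing and rocking animation from BeginPlay.
; Navegar, also called from the construction script, starts two rate-scaled timelines: a slow location lerp and Balanceo, which swings rotation either side of zero.
; The location lerp's end point subtracts a zero offset from the start, so the actor stays in place while rocking.
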(event Custom|navegar
  (bind _returnvalue (Transformation|GetActorLocation))
  (Utilities|FlowControl|Sequence
    (:then_0
      (Variables|Default|Setinicio _returnvalue)
      (Variables|Default|Setfinal (- _returnvalue (Math|Vector|MakeVector 0.0 0.0 0.0)))
      (Components|Timeline|SetPlayRate (Variables|Default|GetTimeline) (/ 1.0 1e+03))
      (bind _newtrack_0 (Timeline|Timeline Play)
        (:Update
          (Transformation|SetActorLocation (Math|Vector|Lerp(Vector) (Variables|Default|Getinicio) (Variables|Default|Getfinal) _newtrack_0) false false))))
    (:then_1
      (Components|Timeline|SetPlayRate (Variables|Default|Getbalanceo) (/ 1.0 5.0))
      (bind _newtrack_1 (Timeline|balanceo Play)
        (:Update
          (if (>= _newtrack_1 0.0)
            (Transformation|SetActorRotation (Math|Rotator|Lerp(Rotator) "0.0,0.0,0.0" "10.000000,0.000000,0.000000" _newtrack_1 true))
            (else
              (Transformation|SetActorRotation (Math|Rotator|Lerp(Rotator) "-10.000000,0.000000,0.000000" "0.000000,0.000000,0.000000" (+ _newtrack_1 1.0) true)))))))))

(event EventBeginPlay
  (CallFunction|Navegar))

(event Collision|EventActorBeginOverlap
  (params (OtherActor :type Actor%20Object%20Reference)))

(event EventTick
  (params (DeltaSeconds :type Float%20%28single-precision%29)))

(fn ConstructionScript
  (CallFunction|Navegar))