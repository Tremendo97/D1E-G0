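; Spawner actor that places a configurable number of BP_Perro enemies at random points inside a box area when play begins.
; The construction script sizes the SpawnArea box from SpawnAreaSize, and BeginPlay loops NumSpawns times, spawning at random points within it.
; After each spawn it casts the player character to BP_Personaje and binds an event to its CrearEnergia dispatcher.
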(event EventBeginPlay
  (bind _spawnarea (Variables|Default|GetSpawnArea))
  (for _index (range 1 (Variables|Default|GetNum%20Spawns))
    (bind _returnvalue (Game|SpawnActorfromClass "/Game/Enemies/BP_Perro.BP_Perro_C" (Math|Transform|MakeTransform (Math|Random|RandomPointinBoundingBox (Transformation|GetWorldLocation _spawnarea) (Components|Box|GetScaledBoxExtent _spawnarea)) "0, 0, 0" "1.000000,1.000000,1.000000") "Undefined" "MultiplyWithRoot" 0 0))
    (bind _asbp_personaje (Utilities|Casting|CastToBP_Personaje (Game|GetPlayerCharacter 0)))
    (EventDispatchers|BindEventtoCrearEnergia _asbp_personaje (EventDispatchers|CreateEvent _returnvalue :!event OnEnergyCreated))))

(fn ConstructionScript
  (Components|Box|SetBoxExtent (Variables|Default|GetSpawnArea) (Variables|Default|GetSpawn%20Area%20Size) true))