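; Rueda enemy that patrols random navmesh points and makes a charge attack when it sees a pawn.
; Tick yaws its cylinder toward the player, while patrol issues a new AI move every two seconds.
; A sighting passes a DoOnce, freezes movement for a wind-up, then sends a fast AIMoveTo overshooting the player's position.
; Successful arrival re-arms detection and resumes patrol; hit pushback is noted as moved to the character Blueprint.
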(event OnSeePawn(PawnSensing)
  (params (Pawn :type Pawn%20Object%20Reference))
  ;[1 1 1] Secuencia de comportamiento
  (Development|PrintString "DETECTADO")
  (Utilities|FlowControl|DoOnce false
    (:Completed
      (Variables|Default|SetMoveRandom false)
      (Utilities|FlowControl|Sequence
        (:then_0
          (Pawn|Components|CharacterMovement|DisableMovement (Variables|Character|GetCharacterMovement)))
        (:then_1
          (Variables|/Script/Engine.CharacterMovementComponent|SetMaxWalkSpeed (Variables|Character|GetCharacterMovement) 1e+03))
        (:then_2
          (CallFunction|Charge))))))

(event Custom|ResetDoOnce
  ;[1 1 1] Secuencia de comportamiento
  (Utilities|FlowControl|DoOnce false) ; enters at Reset
)

(event Custom|MoveToRandomLocation
  ;[1 1 1] Rueda patrulla (movimiento aleatorio en un radio)
  (if (Variables|Default|GetMoveRandom)
    (bind _randomlocation (Class|NavigationSystemV1|GetRandomLocationinNavigableRadius (Transformation|GetActorLocation) 1e+03 0 0))
    (AI|AIMoveTo self _randomlocation 0 5.0 false
      (:then
        (Utilities|FlowControl|Delay 2.0)
        (CallFunction|MovetoRandomLocation)))))

(event Custom|Charge
  (bind _self self)
  (bind _returnvalue (Transformation|GetActorLocation _self))
  (Actor|Tick|SetActorTickEnabled true)
  ;[1 1 1] Charge/Placaje
  (Development|PrintString "Cargando....")
  (Utilities|FlowControl|Delay 5.0)
  (Pawn|Components|CharacterMovement|SetMovementMode (Variables|Character|GetCharacterMovement) "MOVE_Walking" 0)
  (Variables|Default|SetPlayerPosition (Transformation|GetActorLocation (Game|GetPlayerCharacter 0)))
  (AI|AIMoveTo self (+ (* (Math|Vector|Normalize (- (Variables|Default|GetPlayerPosition) _returnvalue)) (+ (Math|Vector|Distance(Vector) _returnvalue (Variables|Default|GetPlayerPosition)) 2e+02)) (Transformation|GetActorLocation self)) 0 5.0 false
    (:OnSuccess
      (Actor|Tick|SetActorTickEnabled true)
      (CallFunction|ResetDoOnce)
      (Variables|/Script/Engine.CharacterMovementComponent|SetMaxWalkSpeed (Variables|Character|GetCharacterMovement) 4e+02)
      (Utilities|FlowControl|RetriggerableDelay 3.0)
      (Variables|Default|SetMoveRandom true)
      (CallFunction|MovetoRandomLocation))))

(event EventBeginPlay
  ;[1 1 1] Rueda patrulla (movimiento aleatorio en un radio)
  (CallFunction|MovetoRandomLocation))

(event EventTick
  (params (DeltaSeconds :type Float%20%28single-precision%29))
  ;[1 1 1] Face Player (SetAim)
  (Transformation|SetWorldRotation (Variables|Default|GetCylinder) (Math|Rotator|MakeRotator 9e+01 0.0 (.Yaw (Math|Rotator|BreakRotator (Math|Rotator|FindLookatRotation (Transformation|GetWorldLocation (Variables|Default|GetCylinder)) (Transformation|GetActorLocation (Game|Player|GetPlayerPawn 0)))))) false false))

(event Collision|EventHit
  (params (MyComp :type Primitive%20Component%20Object%20Reference) (Other :type Actor%20Object%20Reference) (OtherComp :type Primitive%20Component%20Object%20Reference) (bSelfMoved :type Boolean) (HitLocation :type Vector :default "0, 0, 0") (HitNormal :type Vector :default "0, 0, 0") (NormalImpulse :type Vector :default "0, 0, 0") (Hit :type Hit%20Result%20Structure%20%28by%20ref%29))
  ;[1 1 1] Empujar - SE HA MOVIDO AL BP_PERSONAJE
)

(fn ConstructionScript)