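; BP_Rueda is an enemy that wanders to random nearby navigable points and charges the player when it sees a pawn.
; Wandering loops through AI MoveTo with a short pause between moves; a PawnSensing sighting raises walk speed and triggers Charge.
; Charge snapshots the player's position, waits, then moves to a point slightly beyond it along that line.
; Disconnected chase and approach-then-charge variants remain in the graph.
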(event OnSeePawn(PawnSensing)
  (params (Pawn :type Pawn%20Object%20Reference))
  (Utilities|FlowControl|Sequence
    (:then_0
      (Variables|/Script/Engine.CharacterMovementComponent|SetMaxWalkSpeed (Variables|Character|GetCharacterMovement) 6e+02))
    (:then_1
      (CallFunction|Charge))))

(event Custom|MoveToRandomLocation
  (bind _randomlocation (Class|NavigationSystemV1|GetRandomLocationinNavigableRadius (Transformation|GetActorLocation) 1e+03 0 0))
  (AI|AIMoveTo self _randomlocation 0 5.0 false
    (:then
      (Utilities|FlowControl|Delay 2.0)
      (CallFunction|MovetoRandomLocation))))

(event Custom|Charge
  (bind _self self)
  (bind _returnvalue (Transformation|GetActorLocation _self))
  (Variables|Default|SetPlayerPosition (Transformation|GetActorLocation (Game|GetPlayerCharacter 0)))
  (Development|PrintString "Cargando....")
  (Utilities|FlowControl|Delay 2.0)
  (AI|AIMoveTo self (+ (* (Math|Vector|Normalize (- (Variables|Default|GetPlayerPosition) _returnvalue)) (+ (Math|Vector|Distance(Vector) _returnvalue (Variables|Default|GetPlayerPosition)) 1e+02)) (Transformation|GetActorLocation self)) 0 7e+01 false
    (:then
      (Utilities|FlowControl|Delay 0.2))))

(event EventBeginPlay
  (CallFunction|MovetoRandomLocation))

(fn ConstructionScript)