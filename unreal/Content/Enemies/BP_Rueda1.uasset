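; BP_Rueda1 is an enemy that charges at the player when its pawn sensing spots a pawn.
; Charge raises max walk speed cumulatively and uses AIMoveTo toward a point 100 units beyond the player's captured position.
; Its debug-drawn box trace has empty branches, so the result does not affect the charge.
; A separate CustomEvent, uncalled here, prints "Cargando....", waits, then makes the same overshooting move.
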(event OnSeePawn(PawnSensing)
  (params (Pawn :type Pawn%20Object%20Reference))
  (Variables|Default|SetPlayerPosition (Transformation|GetActorLocation (Game|GetPlayerCharacter 0)))
  (CallFunction|Charge))

(event Custom|CustomEvent
  (params (Pawn :type Pawn%20Object%20Reference))
  (bind _self self)
  (bind _returnvalue (Transformation|GetActorLocation _self))
  (Variables|Default|SetPlayerPosition (Transformation|GetActorLocation (Game|GetPlayerCharacter 0)))
  (Development|PrintString "Cargando....")
  (Utilities|FlowControl|Delay 2.0)
  (AI|AIMoveTo self (+ (* (Math|Vector|Normalize (- (Variables|Default|GetPlayerPosition) _returnvalue)) (+ (Math|Vector|Distance(Vector) _returnvalue (Variables|Default|GetPlayerPosition)) 1e+02)) (Transformation|GetActorLocation self)) 0 7e+01 false))

(event Custom|Charge
  (bind _self self)
  (bind _charactermovement (Variables|Character|GetCharacterMovement))
  (bind _playerposition (Variables|Default|GetPlayerPosition))
  (bind _returnvalue (Transformation|GetActorLocation _self))
  (bind (_outhit _returnvalue_2) (Collision|BoxTraceByChannel (Transformation|GetActorLocation) (Variables|Default|GetPlayerPosition) "755.000000,755.000000,300.000000" "0, 0, 0" "TraceTypeQuery1" false 0 "ForDuration"))
  (if _returnvalue_2
    _
    (else
      _))
  (Variables|/Script/Engine.CharacterMovementComponent|SetMaxWalkSpeed _charactermovement (+ (Variables|/Script/Engine.CharacterMovementComponent|GetMaxWalkSpeed _charactermovement) 4e+02))
  (AI|AIMoveTo self (+ (* (Math|Vector|Normalize (- _playerposition _returnvalue)) (+ (Math|Vector|Distance(Vector) _returnvalue _playerposition) 1e+02)) (Transformation|GetActorLocation self)) 0 5.0 false
    (:then
      (Utilities|FlowControl|Delay 4.0))))

(fn ConstructionScript)