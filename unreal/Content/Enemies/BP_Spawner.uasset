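; BP_Spawner is an enemy spawner that places a set number of one enemy type at random points inside a box on BeginPlay.
; The Enemigo selection picks BP_Perro or BP_EnemySemillero, and the construction script sizes the box from SpawnAreaSize.
; Each Perro spawn also binds an event to CrearEnergia on the player's BP_Personaje.
; Semilleros get random yaw and adjust around collisions but always spawn.
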(event EventBeginPlay
  (bind _spawnarea (Variables|Default|GetSpawnArea))
  (bind _spawnarea_2 (Variables|Default|GetSpawnArea))
  (switch Utilities|FlowControl|Switch|SwitchonE_SpawnerSelector (Variables|Default|GetEnemigo)
    (:NewEnumerator0
      (for _index (range 1 (Variables|Default|GetNum%20Spawns))
        (bind _returnvalue (Game|SpawnActorfromClass "/Game/Enemies/BP_Perro.BP_Perro_C" (Math|Transform|MakeTransform (Math|Random|RandomPointinBoundingBox (Transformation|GetWorldLocation _spawnarea_2) (Components|Box|GetScaledBoxExtent _spawnarea_2)) "0, 0, 0" "1.000000,1.000000,1.000000") "Undefined" "MultiplyWithRoot" 0 0))
        (bind _asbp_personaje (Utilities|Casting|CastToBP_Personaje (Game|GetPlayerCharacter 0)))
        (EventDispatchers|BindEventtoCrearEnergia _asbp_personaje (EventDispatchers|CreateEvent _returnvalue :!event OnEnergyCreated))))
    (:NewEnumerator1
      (for _index_2 (range 1 (Variables|Default|GetNum%20Spawns))
        (Game|SpawnActorfromClass "/Game/Enemies/BP_EnemySemillero.BP_EnemySemillero_C" (Math|Transform|MakeTransform (Math|Random|RandomPointinBoundingBox (Transformation|GetWorldLocation _spawnarea) (Components|Box|GetScaledBoxExtent _spawnarea)) (Math|Rotator|MakeRotator 0.0 0.0 (.yaw (Math|Random|RandomRotator false))) "1.000000,1.000000,1.000000") "AdjustIfPossibleButAlwaysSpawn" "MultiplyWithRoot" 0 0)))))

(fn ConstructionScript
  (Components|Box|SetBoxExtent (Variables|Default|GetSpawnArea) (Variables|Default|GetSpawn%20Area%20Size) true))