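; Test actor that drives a material parameter on its Cube when a line trace hit is reported to it.
; LineTraceHit sets the Gate scalar to 1, and a short retriggerable delay returns it to 0 once hits stop arriving.
; Unconnected experiments remain for material swapping, a dynamic instance, a player-facing dot product and a timeline-driven opacity fade, none of which run.
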(event EventBeginPlay)

(event Collision|EventActorBeginOverlap
  (params (OtherActor :type Actor%20Object%20Reference)))

(event EventTick
  (params (DeltaSeconds :type Float%20%28single-precision%29)))

(event EventLineTraceHit
  (bind _cube (Variables|Default|GetCube))
  (Rendering|Material|SetScalarParameterValueonMaterials _cube "Gate" 1.0)
  (Utilities|FlowControl|RetriggerableDelay 0.1)
  (Rendering|Material|SetScalarParameterValueonMaterials _cube "Gate" 0.0))

(fn ConstructionScript)